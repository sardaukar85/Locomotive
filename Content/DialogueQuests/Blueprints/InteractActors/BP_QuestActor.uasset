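; Interactable quest actor that responds only to a player who has the quest set on its ACQuestActor component.
; The Interact-ALL override looks up that quest in the player's AC_QuestsHandler.
; If found, it runs the parent interaction, then calls SetNewQuestInActor on the handler with the Quester, dialogue part zero and itself as finished actor.
; An unconnected AddItem call for a necklace quest item never runs.
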(event EventBeginPlay
  ;[1 1 1] Override Interact Event
  (|CallParentFunction))

(event EventInteract-ALL
  (params (InteractedVariable :type Character%20Object%20Reference))
  ;[1 1 1] Override Interact Event
  (Variables|Default|SetPlayer InteractedVariable)
  (bind _outputpin (Default|FindQuest (Actor|GetComponentbyClass (Variables|Default|GetPlayer) "/Game/DialogueQuests/Blueprints/MapComponents/AC_QuestsHandler.AC_QuestsHandler_C") (.Quest (Utilities|Struct|BreakS_QuestDynam (Variables|/Game/DialogueQuests/Blueprints/Quests/AC_QuestActor.AC_QuestActor_C|GetCurrentQuest (Variables|Default|GetAC_QuestActor))))))
  (if (!= _outputpin -1)
    (|CallParentFunction (Variables|Default|GetPlayer))
    (Default|SetNewQuestinActor (Actor|GetComponentbyClass (Variables|Default|GetPlayer) "/Game/DialogueQuests/Blueprints/MapComponents/AC_QuestsHandler.AC_QuestsHandler_C") (Variables|Default|GetQuester) 0 self)))

(fn ConstructionScript
  (|CallParentFunction))