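; BP_ActorToDestroy is an interactable quest actor that triggers a destroy event when the interacting character is on the preceding subtask.
; HasPreviousTask checks that character's AC_QuestsHandler for the quest in ACQuestActor, at one subtask before this actor's.
; After DestroyEvent, if QuestCharacter reports every enemy killed, it sets the handler's quest to this actor's subtask, passing its reward.
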(event EventBeginPlay
  (|CallParentFunction) ; This node is disabled and will not be called.\nDrag off pins to build functionality.
)

(event Collision|EventActorBeginOverlap
  (params (OtherActor :type Actor%20Object%20Reference)))

(event EventTick
  (params (DeltaSeconds :type Float%20%28single-precision%29)))

(event EventInteract-ALL
  (params (InteractedVariable :type Character%20Object%20Reference))
  (bind _ac_questactor (Variables|Default|GetAC_QuestActor))
  (bind _currentquest (Variables|/Game/DialogueQuests/Blueprints/Quests/AC_QuestActor.AC_QuestActor_C|GetCurrentQuest _ac_questactor))
  (if (CallFunction|HasPreviousTask? InteractedVariable)
    (CallFunction|DestroyEvent)
    (if (Default|KilledEveryEnemy? (Variables|Default|GetQuestCharacter))
      (Default|SetNewQuestSubslot (Actor|GetComponentbyClass InteractedVariable "/Game/DialogueQuests/Blueprints/MapComponents/AC_QuestsHandler.AC_QuestsHandler_C") (.quest _currentquest) (.currentsubtask _currentquest) (Variables|/Game/DialogueQuests/Blueprints/Quests/AC_QuestActor.AC_QuestActor_C|GetReward (Variables|Default|GetAC_QuestActor))))))

(fn ConstructionScript
  (|CallParentFunction))

(fn HasPreviousTask?
  (params (Character :type Actor%20Object%20Reference))
  (bind _returnvalue (Actor|GetComponentbyClass Character "/Game/DialogueQuests/Blueprints/MapComponents/AC_QuestsHandler.AC_QuestsHandler_C"))
  (bind _outputpin (Default|FindQuest _returnvalue (.Quest (Utilities|Struct|BreakS_QuestDynam (Variables|/Game/DialogueQuests/Blueprints/Quests/AC_QuestActor.AC_QuestActor_C|GetCurrentQuest (Variables|Default|GetAC_QuestActor))))))
  (return (and (!= _outputpin -1) (== (.CurrentSubTask (Utilities|Struct|BreakS_QuestDynam (Utilities|Array|Get(acopy) (Variables|/Game/DialogueQuests/Blueprints/MapComponents/AC_QuestsHandler.AC_QuestsHandler_C|GetQuests _returnvalue) _outputpin))) (- (.CurrentSubTask (Utilities|Struct|BreakS_QuestDynam (Variables|/Game/DialogueQuests/Blueprints/Quests/AC_QuestActor.AC_QuestActor_C|GetCurrentQuest (Variables|Default|GetAC_QuestActor)))) 1)))))