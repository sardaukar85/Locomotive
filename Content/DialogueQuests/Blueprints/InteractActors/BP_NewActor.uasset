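; Interactable quest actor that advances a character's quest subtask when interacted with, then destroys itself.
; HasPrepTask looks up the quest from ACQuestActor in the character's AC_QuestsHandler and requires its current subtask to be one before this actor's.
; On a match, it runs parent Interact, calls DestroyEvent and sets the new subtask and reward on the handler.
; DestroyActor runs afterwards even when that check fails.
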(event EventBeginPlay
  (|CallParentFunction) ; This node is disabled and will not be called.\nDrag off pins to build functionality.
)

(event Collision|EventActorBeginOverlap
  (params (OtherActor :type Actor%20Object%20Reference)))

(event EventTick
  (params (DeltaSeconds :type Float%20%28single-precision%29)))

(event EventInteract
  (params (Character :type Character%20Object%20Reference))
  (bind _returnvalue (Actor|GetComponentbyClass Character "/Game/DialogueQuests/Blueprints/MapComponents/AC_QuestsHandler.AC_QuestsHandler_C"))
  (bind _ac_questactor (Variables|Default|GetAC_QuestActor))
  (bind _currentquest (Variables|/Game/DialogueQuests/Blueprints/Quests/AC_QuestActor.AC_QuestActor_C|GetCurrentQuest _ac_questactor))
  (bind (_quest _marked _discovered _currentsubtask) (Utilities|Struct|BreakS_QuestDynam _currentquest))
  (Utilities|FlowControl|Sequence
    (:then_0
      (if (CallFunction|HasPrepTask Character)
        (|CallParentFunction Character)
        (Utilities|IsValid _returnvalue
          (:Is%20Valid
            (CallFunction|DestroyEvent)
            (Default|SetNewQuestSubslot _returnvalue _quest _currentsubtask (Variables|/Game/DialogueQuests/Blueprints/Quests/AC_QuestActor.AC_QuestActor_C|GetReward _ac_questactor))))))
    (:then_1
      (Actor|DestroyActor))))

(fn ConstructionScript
  (|CallParentFunction))

(fn HasPrepTask
  (params (Character :type Actor%20Object%20Reference))
  (bind _returnvalue (Actor|GetComponentbyClass Character "/Game/DialogueQuests/Blueprints/MapComponents/AC_QuestsHandler.AC_QuestsHandler_C"))
  (bind _outputpin (Default|FindQuest _returnvalue (.Quest (Utilities|Struct|BreakS_QuestDynam (Variables|/Game/DialogueQuests/Blueprints/Quests/AC_QuestActor.AC_QuestActor_C|GetCurrentQuest (Variables|Default|GetAC_QuestActor))))))
  (return (and (!= _outputpin -1) (== (.CurrentSubTask (Utilities|Struct|BreakS_QuestDynam (Utilities|Array|Get(acopy) (Variables|/Game/DialogueQuests/Blueprints/MapComponents/AC_QuestsHandler.AC_QuestsHandler_C|GetQuests _returnvalue) _outputpin))) (- (.CurrentSubTask (Utilities|Struct|BreakS_QuestDynam (Variables|/Game/DialogueQuests/Blueprints/Quests/AC_QuestActor.AC_QuestActor_C|GetCurrentQuest (Variables|Default|GetAC_QuestActor)))) 1)))))