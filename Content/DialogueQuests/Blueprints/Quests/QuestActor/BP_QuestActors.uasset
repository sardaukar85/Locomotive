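; World quest actor that advances a character's quest when that character enters its sphere.
; On overlap it takes any character with an AC_QuestsHandler as its owner, under a graph comment marking the overlap as multiplayer.
; If the subtask before its configured one has the required type and SameQuest finds the character on that step, it sets the handler to the configured subtask, passing the ACQuestActor reward.
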(event OnComponentBeginOverlap(Sphere)
  (params (OverlappedComponent :type Primitive%20Component%20Object%20Reference) (OtherActor :type Actor%20Object%20Reference) (OtherComp :type Primitive%20Component%20Object%20Reference) (OtherBodyIndex :type Integer) (bFromSweep :type Boolean) (SweepResult :type Hit%20Result%20Structure%20%28by%20ref%29))
  (bind _ac_questactor (Variables|Default|GetAC_QuestActor))
  (bind _ac_questactor_2 (Variables|Default|GetAC_QuestActor))
  (bind _currentquest (Variables|/Game/DialogueQuests/Blueprints/Quests/AC_QuestActor.AC_QuestActor_C|GetCurrentQuest _ac_questactor))
  (bind _currentquest_2 (Variables|/Game/DialogueQuests/Blueprints/Quests/AC_QuestActor.AC_QuestActor_C|GetCurrentQuest _ac_questactor_2))
  (bind (_quest _marked _discovered _currentsubtask) (Utilities|Struct|BreakS_QuestDynam _currentquest_2))
  (bind (_quest_2 _marked_2 _discovered_2 _currentsubtask_2) (Utilities|Struct|BreakS_QuestDynam _currentquest))
  ;[1 1 1] Multiplayered Overlap
  (bind _ascharacter (Utilities|Casting|CastToCharacter OtherActor))
  (Utilities|IsValid (Actor|GetComponentbyClass _ascharacter "/Game/DialogueQuests/Blueprints/MapComponents/AC_QuestsHandler.AC_QuestsHandler_C")
    (:Is%20Valid
      (Actor|SetOwner _ascharacter)
      (if (Utilities|Enum|Equal(Enum) (.Type (Utilities|Struct|BreakS_SubtaskComplete (Utilities|Array|Get(acopy) (.SubTasksName (Utilities|Struct|BreakS_QuestsMain (CallFunction|GetQuestInfo _quest_2))) (- _currentsubtask_2 1)))) "NewEnumerator2")
        (bind (_res _outputpin) (CallFunction|SameQuest (Actor|GetComponentbyClass _ascharacter "/Game/DialogueQuests/Blueprints/MapComponents/AC_QuestsHandler.AC_QuestsHandler_C")))
        (if (and _res (== _outputpin (- (.CurrentSubTask (Utilities|Struct|BreakS_QuestDynam (Variables|/Game/DialogueQuests/Blueprints/Quests/AC_QuestActor.AC_QuestActor_C|GetCurrentQuest (Variables|Default|GetAC_QuestActor)))) 1)))
          (Default|SetNewQuestSubslot (Actor|GetComponentbyClass _ascharacter "/Game/DialogueQuests/Blueprints/MapComponents/AC_QuestsHandler.AC_QuestsHandler_C") _quest _currentsubtask (Variables|/Game/DialogueQuests/Blueprints/Quests/AC_QuestActor.AC_QuestActor_C|GetReward (Variables|Default|GetAC_QuestActor))))))))

(fn ConstructionScript)

(fn SameQuest
  (params (Target :type AC%20Quests%20Handler%20Object%20Reference))
  (for _array_element (Variables|/Game/DialogueQuests/Blueprints/MapComponents/AC_QuestsHandler.AC_QuestsHandler_C|GetQuests Target)
    (if (Utilities|Name|Equal(Name) (.RowName (Utilities|Struct|BreakDataTableRowHandle (.Quest (Utilities|Struct|BreakS_QuestDynam _array_element)))) (.RowName (Utilities|Struct|BreakDataTableRowHandle (.Quest (Utilities|Struct|BreakS_QuestDynam (Variables|/Game/DialogueQuests/Blueprints/Quests/AC_QuestActor.AC_QuestActor_C|GetCurrentQuest (Variables|Default|GetAC_QuestActor)))))))
      (return true (.CurrentSubTask (Utilities|Struct|BreakS_QuestDynam _array_element)))))
  (return false 0))