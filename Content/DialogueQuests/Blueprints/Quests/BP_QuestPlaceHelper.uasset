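; Quest location marker actor that displays a WB_QuestPoint widget through its Widget component.
; SetNewLocation moves the actor and copies the new location into the widget's Location variable.
; ToggleVisibility and ToggleVis are identical events that show or hide the Widget component without propagating to children.
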(event Custom|ToggleVisibility
  (params (bNewVisibility :type Boolean))
  ;[1 1 1] Toggle Vis
  (Rendering|SetVisibility (Variables|Default|GetWidget) bNewVisibility false))

(event Custom|ToggleVis
  (params (bNewVisibility :type Boolean))
  ;[1 1 1] Toggle Vis
  (Rendering|SetVisibility (Variables|Default|GetWidget) bNewVisibility false))

(event Custom|SetNewLocation
  (params (NewLocation :type Vector))
  ;[1 1 1] New Actor Location
  (Transformation|SetActorLocation NewLocation false false)
  (bind _aswb_quest_point (Utilities|Casting|CastToWB_QuestPoint (UserInterface|GetUserWidgetObject (Variables|Default|GetWidget))))
  (Variables|/Game/DialogueQuests/UI/Widgets/Quests/WB_QuestPoint.WB_QuestPoint_C|SetLocation _aswb_quest_point NewLocation))

(fn ConstructionScript)