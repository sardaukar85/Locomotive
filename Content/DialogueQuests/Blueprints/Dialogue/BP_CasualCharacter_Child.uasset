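; Dialogue NPC, apparently a child of a casual-character base, that offers the player a quest through a two-option conversation.
; Conversation setup adds an accept-or-decline decision; accepting queues lines from ImportantDialogues, chained by finished-dialogue index, while declining ends the dialogue.
; After the last line, it passes its quest actor component's current quest to the player's AC_QuestsHandler and clears MainDialogue.
; Selection only prints the source actor's name.
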(event PressedSelect(Comp_Select)
  (params (Pawn :type BP%20Pawn%20Base%20Object%20Reference) (SourceActor :type Actor%20Object%20Reference) (ImpactLocation :type Vector :default "0, 0, 0") (ImpactComponent :type Actor%20Component%20Object%20Reference))
  (Development|PrintString (Utilities|GetDisplayName SourceActor)))

(event EventBeginPlay
  (|CallParentFunction) ; This node is disabled and will not be called.\nDrag off pins to build functionality.
)

(event Collision|EventActorBeginOverlap
  (params (OtherActor :type Actor%20Object%20Reference))
  (|CallParentFunction OtherActor) ; This node is disabled and will not be called.\nDrag off pins to build functionality.
)

(event EventTick
  (params (DeltaSeconds :type Float%20%28single-precision%29))
  (|CallParentFunction DeltaSeconds) ; This node is disabled and will not be called.\nDrag off pins to build functionality.
)

(event EventCurrentDialogueFinished
  (params (Index :type Integer))
  (bind _playerchar (Variables|Default|GetPlayerChar))
  (bind _returnvalue (Actor|GetComponentbyClass _playerchar "/Game/DialogueQuests/Blueprints/MapComponents/AC_QuestsHandler.AC_QuestsHandler_C"))
  (switch int Index
    (:0
      (CallFunction|AddNewDialogue 1 (.DialogueInfo (CallFunction|GetDialogueInfo (Variables|Default|GetImportantDialogues) 1))))
    (:1
      (CallFunction|DialogueFinished)
      (Utilities|IsValid _returnvalue
        (:Is%20Valid
          (Default|AddNewQuest _returnvalue (Variables|/Game/DialogueQuests/Blueprints/Quests/AC_QuestActor.AC_QuestActor_C|GetCurrentQuest (Variables|Default|GetAC_QuestActor)))
          (Variables|Default|SetMainDialogue? false))))))

(event EventMadeDecision
  (params (Decision :type Integer) (Option :type Integer))
  (switch int Option
    (:1
      (CallFunction|AddNewDialogue 0 (.DialogueInfo (CallFunction|GetDialogueInfo (Variables|Default|GetImportantDialogues)))))
    (:2
      (CallFunction|DialogueFinished))))

(event EventAfterConversationSetup
  (CallFunction|AddDecision 0 (Utilities|Struct|MakeS_OptionInfo (.DialogueInfo (CallFunction|GetDialogueInfo (Variables|Default|GetImportantDialogues))) (Utilities|Array|MakeArray (Utilities|Struct|MakeS_DialogueOption "I Will" 0 "NewEnumerator4" "(R=0.000000,G=0.000000,B=0.000000,A=0.000000)") (Utilities|Struct|MakeS_DialogueOption "No" 0 "NewEnumerator0" "(R=0.000000,G=0.000000,B=0.000000,A=0.000000)")) false 10)))

(fn ConstructionScript
  (|CallParentFunction))