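; BP_CameraHelper is a dialogue camera helper that picks an unobstructed view camera from two candidates.
; GetViewCamera pairs each camera with a sphere and tests a random pair for overlapping StaticMeshActors.
; Blocked pairs are removed and the random pick repeats until one is clear or none remain.
; A clear camera is set inactive and returned with a true result; otherwise the result is false.
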(fn ConstructionScript)

(fn GetViewCamera
  ;[1 1 1] Select And Configure Camera
  (Variables|Default|SetSpheresArray (Utilities|Array|MakeArray (Variables|Default|GetSphere3) (Variables|Default|GetSphere2)))
  (Variables|Default|SetCamerasArray (Utilities|Array|MakeArray (Variables|Default|GetCamera) (Variables|Default|GetCamera1)))
  (Variables|Default|SetCurrentRandomNumber (Math|Random|RandomIntegerinRange 0 (- (Utilities|Array|Length (Variables|Default|GetCamerasArray)) 1)) :!label _label)
  (if (> (Utilities|Array|Length (Collision|GetOverlappingActors (Utilities|Array|Get(acopy) (Variables|Default|GetSpheresArray) (Variables|Default|GetCurrentRandomNumber)) "/Script/Engine.StaticMeshActor" :!class /Script/Engine.PrimitiveComponent)) 0)
    (Utilities|Array|RemoveIndex (Variables|Default|GetCamerasArray) (Variables|Default|GetCurrentRandomNumber))
    (Utilities|Array|RemoveIndex (Variables|Default|GetSpheresArray) (Variables|Default|GetCurrentRandomNumber))
    (if (> (Utilities|Array|Length (Variables|Default|GetCamerasArray)) 0)
      (goto _label)
      (else
        (return false 0)))
    (else
      (Components|Activation|SetActive (Utilities|Array|Get(acopy) (Variables|Default|GetCamerasArray) (Variables|Default|GetCurrentRandomNumber)) false false)
      (return true (Utilities|Array|Get(acopy) (Variables|Default|GetCamerasArray) (Variables|Default|GetCurrentRandomNumber))))))