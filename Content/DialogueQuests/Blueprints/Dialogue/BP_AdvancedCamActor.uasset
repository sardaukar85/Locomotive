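; BP_AdvancedCamActor is a dialogue camera actor that animates its camera component toward the relative location and rotation of a NextCameraPoint.
; StartAnimation caches the camera's current relative transform and opens a Tick gate that lerps toward the target.
; Alpha grows by a fixed step per frame, so speed depends on frame rate, and is never reset here.
; StopAnimation closes the gate, automatically at 0.9 alpha, short of the full target.
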(event Custom|StartAnimation
  (bind _nextcamerapoint (Variables|Default|GetNextCameraPoint))
  (bind _cameracomponent (Variables|CameraActor|GetCameraComponent))
  (Variables|Default|SetStartLocation (Variables|/Script/Engine.SceneComponent|GetRelativeLocation _cameracomponent))
  (Variables|Default|SetStartRotation (Variables|/Script/Engine.SceneComponent|GetRelativeRotation _cameracomponent))
  (Utilities|FlowControl|Gate true) ; enters at Open
)

(event Custom|StopAnimation
  (bind _nextcamerapoint (Variables|Default|GetNextCameraPoint))
  (Utilities|FlowControl|Gate true) ; enters at Close
)

(event EventTick
  (params (DeltaSeconds :type Float%20%28single-precision%29))
  (bind _nextcamerapoint (Variables|Default|GetNextCameraPoint))
  (Utilities|FlowControl|Gate true
    (:Exit
      (Variables|Default|SetCurrentAlpha (+ (Variables|Default|GetCurrentAlpha) 0.008))
      (Transformation|SetRelativeLocationAndRotation (Variables|CameraActor|GetCameraComponent) (Math|Vector|Lerp(Vector) (Variables|Default|GetStartLocation) (Variables|/Script/Engine.SceneComponent|GetRelativeLocation _nextcamerapoint) (Variables|Default|GetCurrentAlpha)) (Math|Rotator|Lerp(Rotator) (Variables|Default|GetStartRotation) (Variables|/Script/Engine.SceneComponent|GetRelativeRotation _nextcamerapoint) (Variables|Default|GetCurrentAlpha)) false false)
      (if (>= (Variables|Default|GetCurrentAlpha) 0.9)
        (CallFunction|StopAnimation)))))

(fn ConstructionScript)