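; Blueprint function library of shared helpers for the dialogue and quest system.
; Getters resolve row handles into quest, item, dialogue, smalltalk and world actor data, and scan data tables for emblem icons and quest colors by type.
; SaveGame triggers saving on the target's quest, inventory, money and experience components, then records every BP_InteractActor's state in SaveItems.
; TogglePause creates or removes the pause widget through a by-ref variable.
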(fn GetQuestInfo
  (params (Item :type Data%20Table%20Row%20Handle%20Structure))
  (bind (_datatable _rowname) (Utilities|Struct|BreakDataTableRowHandle Item))
  (bind _returnvalue (Utilities|GetDataTableRow _datatable _rowname)
    (:then
      (return _returnvalue))))

(fn GetItemInfo
  (params (Item :type Data%20Table%20Row%20Handle%20Structure))
  (bind _returnvalue (Utilities|GetDataTableRow "/Game/DialogueQuests/Blueprints/Information/Items/DT_Items.DT_Items" (.RowName (Utilities|Struct|BreakDataTableRowHandle Item)))
    (:then
      (return _returnvalue))))

(fn GetDialogueInfo
  (params (Dialogue :type S%20Dialogue%20Info%20Dynamic%20Structure))
  (bind _dialogue (Utilities|Struct|BreakS_DialogueInfoDynamic Dialogue))
  (bind (_datatable _rowname) (Utilities|Struct|BreakDataTableRowHandle _dialogue))
  (bind _returnvalue (Utilities|GetDataTableRow _datatable _rowname)
    (:then
      (return _returnvalue))))

(fn GetSmalltalkInfo
  (params (Title :type S%20Character%20Text%20Dynamic%20Structure%20%28by%20ref%29))
  (bind _dialogue (Utilities|Struct|BreakS_CharacterTextDynamic Title))
  (bind (_datatable _rowname) (Utilities|Struct|BreakDataTableRowHandle _dialogue))
  (bind _returnvalue (Utilities|GetDataTableRow _datatable _rowname)
    (:then
      (return _returnvalue))))

(fn SaveGame
  (params (Target :type Actor%20Object%20Reference))
  (Default|SaveQuests (Actor|GetComponentbyClass Target "/Game/DialogueQuests/Blueprints/MapComponents/AC_QuestsHandler.AC_QuestsHandler_C"))
  (Default|SaveInventory (Actor|GetComponentbyClass Target "/Game/DialogueQuests/Blueprints/MapComponents/PlayerState/AC_Inventory.AC_Inventory_C"))
  (Default|SaveMoney (Actor|GetComponentbyClass Target "/Game/DialogueQuests/Blueprints/MapComponents/PlayerState/AC_MoneySystem.AC_MoneySystem_C"))
  (Default|SaveExp (Actor|GetComponentbyClass Target "/Game/DialogueQuests/Blueprints/MapComponents/PlayerState/AC_ExpSystem.AC_ExpSystem_C"))
  (bind _outactors (Actor|GetAllActorsOfClass Target "/Game/DialogueQuests/Blueprints/InteractActors/BP_InteractActor.BP_InteractActor_C"))
  (for _array_element _outactors
    (bind _returnvalue (Game|GetCurrentLevelName _array_element))
    (Utilities|Array|Add (LocalVariables|GetSaveItems) (Utilities|Struct|MakeS_SaveWorldItem (Variables|/Game/DialogueQuests/Blueprints/InteractActors/BP_InteractActor.BP_InteractActor_C|GetSpawned? _array_element) (Variables|/Game/DialogueQuests/Blueprints/InteractActors/BP_InteractActor.BP_InteractActor_C|GetisDestroyed _array_element) (Variables|/Game/DialogueQuests/Blueprints/InteractActors/BP_InteractActor.BP_InteractActor_C|GetBlocked _array_element) 0 (Variables|/Game/DialogueQuests/Blueprints/InteractActors/BP_InteractActor.BP_InteractActor_C|GetQuestCharacter _array_element) (Transformation|GetActorLocation _array_element) (Variables|/Game/DialogueQuests/Blueprints/InteractActors/BP_InteractActor.BP_InteractActor_C|GetItem _array_element) (Variables|/Game/DialogueQuests/Blueprints/InteractActors/BP_InteractActor.BP_InteractActor_C|GetMultipleItems _array_element) (Variables|/Game/DialogueQuests/Blueprints/InteractActors/BP_InteractActor.BP_InteractActor_C|GetWorldActor _array_element) (Variables|/Game/DialogueQuests/Blueprints/InteractActors/BP_InteractActor.BP_InteractActor_C|GetType _array_element) (Utilities|GetClass _array_element) (Variables|/Game/DialogueQuests/Blueprints/InteractActors/BP_InteractActor.BP_InteractActor_C|GetBlockOrDelete _array_element) _array_element _returnvalue))))

(fn GetEmplembyType
  (params (InputPin :type E_Region%20Enum :default "NewEnumerator0"))
  (bind _outrownames (DataTable|GetDataTableRowNames "/Game/DialogueQuests/Blueprints/Quests/Area/DT_EmblemType.DT_EmblemType"))
  (for _array_element _outrownames
    (bind _returnvalue (Utilities|GetDataTableRow "/Game/DialogueQuests/Blueprints/Quests/Area/DT_EmblemType.DT_EmblemType" _array_element)
      (:then
        (if (Utilities|Enum|Equal(Enum) (.Area (Utilities|Struct|BreakS_EmblemType _returnvalue)) InputPin)
          (return (.Icon (Utilities|Struct|BreakS_EmblemType _returnvalue))))))))

(fn GetQuestColorbyType
  (params (InputPin :type E_QuestType%20Enum :default "NewEnumerator0"))
  (bind _outrownames (DataTable|GetDataTableRowNames "/Game/DialogueQuests/Blueprints/Quests/Area/DT_QuestColor.DT_QuestColor"))
  (for _array_element _outrownames
    (bind _returnvalue (Utilities|GetDataTableRow "/Game/DialogueQuests/Blueprints/Quests/Area/DT_QuestColor.DT_QuestColor" _array_element)
      (:then
        (if (Utilities|Enum|Equal(Enum) (.QuestType (Utilities|Struct|BreakS_QuestColor _returnvalue)) InputPin)
          (return (.Color (Utilities|Struct|BreakS_QuestColor _returnvalue))))))))

(fn GetWorldActorInfo
  (params (Item :type Data%20Table%20Row%20Handle%20Structure))
  (bind (_datatable _rowname) (Utilities|Struct|BreakDataTableRowHandle Item))
  (bind _returnvalue (Utilities|GetDataTableRow _datatable _rowname)
    (:then
      (return _returnvalue))))

(fn TogglePause
  (params (Widget :type WB%20Pause%20Object%20Reference%20%28by%20ref%29))
  (Utilities|IsValid Widget
    (:Is%20Valid
      (Widget|RemovefromParent Widget)
      (|SetBy-RefVar Widget))
    (:Is%20Not%20Valid
      (bind _returnvalue (UserInterface|CreateWidget "/Game/DialogueQuests/UI/Widgets/Menu/WB_Pause.WB_Pause_C"))
      (|SetBy-RefVar Widget _returnvalue)
      (UserInterface|Viewport|AddtoViewport Widget 0))))