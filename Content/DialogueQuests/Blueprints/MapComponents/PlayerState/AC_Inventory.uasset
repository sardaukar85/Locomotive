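; Inventory component for the player character that stores item slots and handles stacking, swapping, modifications, quality repair and weight.
; On possessed pawns, a delayed BeginPlay loads the inventory from a save slot or calls InitialEquip.
; AddItem tops up matching stacks before using empty slots, and helpers toggle the menu, derive walk-speed curve values from excess weight and trace drop points.
; Equip, use, quick-item and UI-refresh functions are empty stubs.
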(event Custom|Initialize
  (params (MainWidget :type WB%20Main%20Gameplay%20Menu%20Object%20Reference))
  ;[1 1 1] Initialize player
  (Variables|Default|SetMainWidget MainWidget)
  (bind _ascharacter (Utilities|Casting|CastToCharacter (Components|GetOwner)))
  (bind _output_get (Variables|Default|SetPlayer _ascharacter))
  (bind _asplayer_controller (Utilities|Casting|CastToPlayerController (Pawn|GetController _output_get)))
  (Variables|Default|SetPlayerController _asplayer_controller)
  (Variables|Default|SetCurrentWeight (Math|Float|Truncate (CallFunction|GetCurrentWeight)))
  (Variables|Default|SetCasualWalkSpeed (Variables|/Script/Engine.CharacterMovementComponent|GetMaxWalkSpeed (Actor|GetComponentbyClass (Variables|Default|GetPlayer) "/Script/Engine.CharacterMovementComponent"))))

(event Custom|SetNewWidgetActive
  (params (CurrentMenuIndex :type Integer))
  (bind _mainwidget (Variables|Default|GetMainWidget))
  (bind _wb_maintopgui (Variables|/Game/DialogueQuests/UI/Widgets/Menu/WB_MainGameplayMenu.WB_MainGameplayMenu_C|GetWB_MainTopGUI _mainwidget))
  ;[1 1 1] Set Inventory Widget Active
  (Appearance|SetColorandOpacity (Variables|/Game/DialogueQuests/Blueprints/WidgetHandler/AC_MainWidgetHandler.AC_MainWidgetHandler_C|GetWB_MainGUI (Actor|GetComponentbyClass (Components|GetOwner) "/Game/DialogueQuests/Blueprints/WidgetHandler/AC_MainWidgetHandler.AC_MainWidgetHandler_C")) "(R=1.000000,G=1.000000,B=1.000000,A=1.000000)" :!class /Script/UMG.UserWidget)
  (CallFunction|ToggleInventory)
  (Utilities|IsValid _mainwidget
    (:Is%20Valid
      (Variables|/Game/DialogueQuests/UI/Widgets/MainGameplayGUI/WB_MainTopGUI.WB_MainTopGUI_C|SetCurrentMenuIndex _wb_maintopgui CurrentMenuIndex)
      (Default|Update _wb_maintopgui)
      (Default|SetActiveWidgetIndex _wb_maintopgui))))

(event Custom|ToggleInventory
  (bind _playercontroller (Variables|Default|GetPlayerController))
  (bind _mainwidget (Variables|Default|GetMainWidget))
  (bind _mainwidget_2 (Variables|Default|GetMainWidget))
  ;[1 1 1] Toggle inventory logic
  (Utilities|IsValid _mainwidget
    (:Is%20Valid
      (if (Utilities|Enum|Equal(Enum) (Widget|GetVisibility _mainwidget) "Visible")
        (Widget|SetVisibility (Variables|Default|GetMainWidget) "Hidden")
        (Input|SetInputModeGameOnly _playercontroller)
        (Variables|/Script/Engine.PlayerController|SetbShowMouseCursor _playercontroller false)
        (else
          (Widget|SetVisibility (Variables|Default|GetMainWidget) "Visible")
          (Input|SetInputModeUIOnly _playercontroller _mainwidget_2 "DoNotLock")
          (Variables|/Script/Engine.PlayerController|SetbShowMouseCursor _playercontroller true)
          (Class|Widget|SetUserFocus _mainwidget_2 (Variables|Default|GetPlayerController)))))))

(event EventBeginPlay
  ;[1 1 1] Begin Play
  (bind _aspawn (Utilities|Casting|CastToPawn (Components|GetOwner)))
  (if (Class|Pawn|IsControlled _aspawn)
    (Utilities|FlowControl|Delay 1.2)
    (bind _returnvalue (SaveGame|DoesSaveGameExist (Variables|Default|GetInventorySlot)))
    (if _returnvalue
      (Save|LoadInventory)
      (elif (> (Utilities|Array|Length (Variables|Inventory|GetInitialEquipment)) 0)
        (CallFunction|InitialEquip)))))

(fn AddItems
  (params (Items :type Array%20of%20S%20Items%20Inventory%20Structures))
  (for _array_element Items
    (Utilities|Array|Add (Variables|Inventory|GetInventory) _array_element))
  (CallFunction|UpdateInventory))

(fn UpdateInventory)

(fn LoadInventory
  (bind _returnvalue (SaveGame|DoesSaveGameExist (Variables|Default|GetInventorySlot)))
  (if _returnvalue
    (bind _returnvalue_2 (SaveGame|LoadGamefromSlot (Variables|Default|GetInventorySlot)))
    (bind _asbp_save_inventory (Utilities|Casting|CastToBP_Save_Inventory _returnvalue_2))
    (Variables|Inventory|SetInventory (Variables|/Game/DialogueQuests/Blueprints/MapComponents/ComponentsSaves/BP_Save_Inventory.BP_Save_Inventory_C|GetsInventory _asbp_save_inventory))))

(fn SaveInventory
  (bind _returnvalue (SaveGame|DoesSaveGameExist (Variables|Default|GetInventorySlot)))
  (if _returnvalue
    (bind _returnvalue_2 (SaveGame|LoadGamefromSlot (Variables|Default|GetInventorySlot)))
    (bind _asbp_save_inventory (Utilities|Casting|CastToBP_Save_Inventory _returnvalue_2))
    (Variables|Default|SetSaveGAme _asbp_save_inventory)
    (else
      (bind _returnvalue_3 (SaveGame|CreateSaveGameObject "/Game/DialogueQuests/Blueprints/MapComponents/ComponentsSaves/BP_Save_Inventory.BP_Save_Inventory_C"))
      (Variables|Default|SetSaveGAme _returnvalue_3)))
  (Variables|/Game/DialogueQuests/Blueprints/MapComponents/ComponentsSaves/BP_Save_Inventory.BP_Save_Inventory_C|SetsInventory (Variables|Default|GetSaveGAme) (Variables|Inventory|GetInventory))
  (SaveGame|SaveGametoSlot (Variables|Default|GetSaveGAme) (Variables|Default|GetInventorySlot)))

(fn SwapItems
  (params (Index_0 :type Integer) (Index_1 :type Integer))
  (LocalVariables|SetL_Index_0 Index_0)
  (LocalVariables|SetL_Index_1 Index_1)
  (if (!= (LocalVariables|GetL_Index_0) (LocalVariables|GetL_Index_1))
    (LocalVariables|SetL_Temp (Utilities|Array|Get(acopy) (Variables|Inventory|GetInventory) (LocalVariables|GetL_Index_0)))
    (Utilities|Array|SetArrayElem (Variables|Inventory|GetInventory) (LocalVariables|GetL_Index_0) (Utilities|Array|Get(acopy) (Variables|Inventory|GetInventory) (LocalVariables|GetL_Index_1)) true)
    (Utilities|Array|SetArrayElem (Variables|Inventory|GetInventory) (LocalVariables|GetL_Index_1) (LocalVariables|GetL_Temp) true)
    (CallFunction|UpdateInventory)))

(fn RemoveItem
  (params (Ammount :type Integer) (Index :type Integer))
  (bind _inventory (Variables|Inventory|GetInventory))
  (LocalVariables|SetL_Index Index)
  (LocalVariables|SetL_Amount Ammount)
  (if (<= (- (.Amount (Utilities|Struct|BreakS_ItemsInventory (Utilities|Array|Get(acopy) (Variables|Inventory|GetInventory) Index))) Ammount) 0)
    (Utilities|Array|RemoveIndex (Variables|Inventory|GetInventory) (LocalVariables|GetL_Index))
    (else
      (Utilities|Array|SetArrayElem _inventory (LocalVariables|GetL_Index) (Utilities|Struct|MakeS_ItemsInventory (.Item (Utilities|Struct|BreakS_ItemsInventory (Utilities|Array|Get(acopy) _inventory (LocalVariables|GetL_Index)))) (- (.Amount (Utilities|Struct|BreakS_ItemsInventory (Utilities|Array|Get(acopy) _inventory (LocalVariables|GetL_Index)))) (LocalVariables|GetL_Amount)) (.Modifications (Utilities|Struct|BreakS_ItemsInventory (Utilities|Array|Get(acopy) _inventory (LocalVariables|GetL_Index)))) (.SellerInformation (Utilities|Struct|BreakS_ItemsInventory (Utilities|Array|Get(acopy) _inventory (LocalVariables|GetL_Index))))) true))))

(fn AddModification
  (params (Modification :type Data%20Table%20Row%20Handle%20Structure) (Index :type Integer))
  (bind _output_get (LocalVariables|SetL_TempSlot (Utilities|Array|Get(acopy) (Variables|Inventory|GetInventory) Index)))
  (Utilities|Array|Add (.Modifications (Utilities|Struct|BreakS_ItemsInventory _output_get)) Modification)
  (Utilities|Array|SetArrayElem (Variables|Inventory|GetInventory) Index (LocalVariables|GetL_TempSlot)))

(fn HasItem?
  (params (S_ItemsInventory :type S%20Items%20Inventory%20Structure%20%28by%20ref%29))
  (for (_array_element _array_index) (Variables|Inventory|GetInventory)
    (if (and (< (.Amount (Utilities|Struct|BreakS_ItemsInventory _array_element)) (.MaxInSlot (Utilities|Struct|BreakS_ItemStatic (CallFunction|GetItemInfo (.Item (Utilities|Struct|BreakS_ItemsInventory _array_element)))))) (Utilities|Name|Equal(Name) (.RowName (Utilities|Struct|BreakDataTableRowHandle (.Item (Utilities|Struct|BreakS_ItemsInventory _array_element)))) (.RowName (Utilities|Struct|BreakDataTableRowHandle (.Item (Utilities|Struct|BreakS_ItemsInventory S_ItemsInventory))))))
      (return (and (< (.Amount (Utilities|Struct|BreakS_ItemsInventory _array_element)) (.MaxInSlot (Utilities|Struct|BreakS_ItemStatic (CallFunction|GetItemInfo (.Item (Utilities|Struct|BreakS_ItemsInventory _array_element)))))) (Utilities|Name|Equal(Name) (.RowName (Utilities|Struct|BreakDataTableRowHandle (.Item (Utilities|Struct|BreakS_ItemsInventory _array_element)))) (.RowName (Utilities|Struct|BreakDataTableRowHandle (.Item (Utilities|Struct|BreakS_ItemsInventory S_ItemsInventory)))))) _array_index)))
  (return false 0))

(fn SameType?
  (params (IndexDropped :type Integer) (Index :type Integer))
  (bind _inventory (Variables|Inventory|GetInventory))
  (bind _output (Utilities|Array|Get(acopy) _inventory IndexDropped))
  (bind (_item _amount) (Utilities|Struct|BreakS_ItemsInventory _output))
  (return (and (Utilities|Name|Equal(Name) (.RowName (Utilities|Struct|BreakDataTableRowHandle _item)) (.RowName (Utilities|Struct|BreakDataTableRowHandle (.Item (Utilities|Struct|BreakS_ItemsInventory (Utilities|Array|Get(acopy) (Variables|Inventory|GetInventory) Index)))))) (< _amount (.MaxInSlot (Utilities|Struct|BreakS_ItemStatic (CallFunction|GetItemInfo _item)))))))

(fn SplitItemsAmount
  (params (Index :type Integer) (IndexDrppped :type Integer))
  (LocalVariables|SetL_Index Index)
  (LocalVariables|SetL_DroppedIndex IndexDrppped)
  (if (> (- (.MaxInSlot (Utilities|Struct|BreakS_ItemStatic (CallFunction|GetItemInfo (.Item (Utilities|Struct|BreakS_ItemsInventory (Utilities|Array|Get(acopy) (Variables|Inventory|GetInventory) (LocalVariables|GetL_Index))))))) (.Amount (Utilities|Struct|BreakS_ItemsInventory (Utilities|Array|Get(acopy) (Variables|Inventory|GetInventory) (LocalVariables|GetL_Index))))) 0)
    (if (< (- (.Amount (Utilities|Struct|BreakS_ItemsInventory (Utilities|Array|Get(acopy) (Variables|Inventory|GetInventory) (LocalVariables|GetL_DroppedIndex)))) (- (.MaxInSlot (Utilities|Struct|BreakS_ItemStatic (CallFunction|GetItemInfo (.Item (Utilities|Struct|BreakS_ItemsInventory (Utilities|Array|Get(acopy) (Variables|Inventory|GetInventory) (LocalVariables|GetL_Index))))))) (.Amount (Utilities|Struct|BreakS_ItemsInventory (Utilities|Array|Get(acopy) (Variables|Inventory|GetInventory) (LocalVariables|GetL_Index)))))) 0)
      ;[1 1 1] If In A dropped amount less items then in (max-indexAmount)
      (Manipulate|SetAmmounttoSlot (+ (.Amount (Utilities|Struct|BreakS_ItemsInventory (Utilities|Array|Get(acopy) (Variables|Inventory|GetInventory) (LocalVariables|GetL_Index)))) (.Amount (Utilities|Struct|BreakS_ItemsInventory (Utilities|Array|Get(acopy) (Variables|Inventory|GetInventory) (LocalVariables|GetL_DroppedIndex))))) (LocalVariables|GetL_Index))
      (Utilities|Array|RemoveIndex (Variables|Inventory|GetInventory) (LocalVariables|GetL_DroppedIndex))
      (else
        ;[1 1 1] If in a dropped amound moer then in(max-indexAmount)
        (Manipulate|SetAmmounttoSlot (- (.Amount (Utilities|Struct|BreakS_ItemsInventory (Utilities|Array|Get(acopy) (Variables|Inventory|GetInventory) (LocalVariables|GetL_DroppedIndex)))) (- (.MaxInSlot (Utilities|Struct|BreakS_ItemStatic (CallFunction|GetItemInfo (.Item (Utilities|Struct|BreakS_ItemsInventory (Utilities|Array|Get(acopy) (Variables|Inventory|GetInventory) (LocalVariables|GetL_Index))))))) (.Amount (Utilities|Struct|BreakS_ItemsInventory (Utilities|Array|Get(acopy) (Variables|Inventory|GetInventory) (LocalVariables|GetL_Index)))))) (LocalVariables|GetL_DroppedIndex))
        (Manipulate|SetAmmounttoSlot (.MaxInSlot (Utilities|Struct|BreakS_ItemStatic (CallFunction|GetItemInfo (.Item (Utilities|Struct|BreakS_ItemsInventory (Utilities|Array|Get(acopy) (Variables|Inventory|GetInventory) (LocalVariables|GetL_Index))))))) (LocalVariables|GetL_Index))))))

(fn SetAmmounttoSlot
  (params (Amount :type Integer) (Index :type Integer))
  (bind _output_get (LocalVariables|SetL_TempInvSlot (Utilities|Array|Get(acopy) (Variables|Inventory|GetInventory) Index)))
  (Utilities|Struct|SetmembersinS_ItemsInventory _output_get Amount)
  (Utilities|Array|SetArrayElem (Variables|Inventory|GetInventory) Index (LocalVariables|GetL_TempInvSlot) true))

(fn AddItem
  (params (Item :type S%20Items%20Inventory%20Structure))
  (LocalVariables|SetL_Item Item)
  (LocalVariables|SetL_Amount (.Amount (Utilities|Struct|BreakS_ItemsInventory Item)))
  (bind _array_index (Utilities|HasItem (LocalVariables|GetL_Item) :!label _label)
    (:true
      (LocalVariables|SetL_arrayIndex _array_index)
      (if (.Return (CallFunction|MoreThanCanSlotKeep? (LocalVariables|GetL_Amount) (LocalVariables|GetL_arrayIndex)))
        (LocalVariables|SetL_Amount (- (LocalVariables|GetL_Amount) (- (.MaxInSlot (Utilities|Struct|BreakS_ItemStatic (CallFunction|GetItemInfo (.Item (Utilities|Struct|BreakS_ItemsInventory (Utilities|Array|Get(acopy) (Variables|Inventory|GetInventory) (LocalVariables|GetL_arrayIndex))))))) (.Amount (Utilities|Struct|BreakS_ItemsInventory (Utilities|Array|Get(acopy) (Variables|Inventory|GetInventory) (LocalVariables|GetL_arrayIndex)))))))
        (Manipulate|SetAmmounttoSlot (.MaxInSlot (Utilities|Struct|BreakS_ItemStatic (CallFunction|GetItemInfo (.Item (Utilities|Struct|BreakS_ItemsInventory (Utilities|Array|Get(acopy) (Variables|Inventory|GetInventory) (LocalVariables|GetL_arrayIndex))))))) (LocalVariables|GetL_arrayIndex))
        (goto _label)
        (else
          (Manipulate|SetAmmounttoSlot (.Sum (CallFunction|MoreThanCanSlotKeep? (LocalVariables|GetL_Amount) (LocalVariables|GetL_arrayIndex))) (LocalVariables|GetL_arrayIndex)))))
    (:Else
      (bind _slotindex (Utilities|HasEmptySlots)
        (:true
          (Utilities|Array|SetArrayElem (Variables|Inventory|GetInventory) _slotindex (Utilities|Struct|MakeS_ItemsInventory (.Item (Utilities|Struct|BreakS_ItemsInventory (LocalVariables|GetL_Item))) (LocalVariables|GetL_Amount) (.Modifications (Utilities|Struct|BreakS_ItemsInventory (LocalVariables|GetL_Item))) (.SellerInformation (Utilities|Struct|BreakS_ItemsInventory (LocalVariables|GetL_Item))) (.Qualoty (Utilities|Struct|BreakS_ItemsInventory (LocalVariables|GetL_Item))))))
        (:false
          (Utilities|Array|Add (Variables|Inventory|GetInventory) (Utilities|Struct|MakeS_ItemsInventory (.Item (Utilities|Struct|BreakS_ItemsInventory (LocalVariables|GetL_Item))) (LocalVariables|GetL_Amount) (.Modifications (Utilities|Struct|BreakS_ItemsInventory (LocalVariables|GetL_Item))) (.SellerInformation (Utilities|Struct|BreakS_ItemsInventory (LocalVariables|GetL_Item))) (.Qualoty (Utilities|Struct|BreakS_ItemsInventory (LocalVariables|GetL_Item))))))))))

(fn MoreThanCanSlotKeep?
  (params (Amount :type Integer) (ItemIndex :type Integer))
  (bind _inventory (Variables|Inventory|GetInventory))
  (bind _output (Utilities|Array|Get(acopy) _inventory ItemIndex))
  (bind (_item _amount) (Utilities|Struct|BreakS_ItemsInventory _output))
  (bind _returnvalue (+ Amount _amount))
  (return (> _returnvalue (.MaxInSlot (Utilities|Struct|BreakS_ItemStatic (CallFunction|GetItemInfo _item)))) _returnvalue))

(fn GetSpawnItemPlace
  (bind _dropbox (Variables|Default|GetDropBox))
  (bind _returnvalue (Transformation|GetWorldLocation _dropbox))
  (bind _returnvalue_2 (Components|Box|GetScaledBoxExtent _dropbox))
  (bind _returnvalue_3 (Math|Random|RandomPointinBoundingBox _returnvalue _returnvalue_2))
  (bind (_x _y _z) (Math|Vector|BreakVector _returnvalue_3))
  (bind _outhit (Collision|LineTraceByChannel _returnvalue_3 (Math|Vector|MakeVector _x _y (- _z 5e+02)) "TraceTypeQuery1" false 0 "None"))
  (return (Math|Conversions|ToTransform(Vector) (.Location (Collision|BreakHitResult _outhit)))))

(fn GetCurrentWeight
  (for _array_element (Variables|Inventory|GetInventory)
    (LocalVariables|SetL_CurrentWeight (+ (LocalVariables|GetL_CurrentWeight) (* (.Amount (Utilities|Struct|BreakS_ItemsInventory _array_element)) (.Weight (Utilities|Struct|BreakS_ItemStatic (CallFunction|GetItemInfo (.Item (Utilities|Struct|BreakS_ItemsInventory _array_element)))))))))
  (return (LocalVariables|GetL_CurrentWeight)))

(fn GetEmptySlot
  (for (_array_element _array_index) (Variables|Inventory|GetInventory)
    (Utilities|IsValid (.DataTable (Utilities|Struct|BreakDataTableRowHandle (.Item (Utilities|Struct|BreakS_ItemsInventory _array_element))))
      (:Is%20Not%20Valid
        (return true _array_index))))
  (return false 0))

(fn IsMainInventory
  (bind _returnvalue (Components|GetOwner))
  (bind _returnvalue_2 (Actor|GetComponentbyClass _returnvalue "/Game/DialogueQuests/Blueprints/WidgetHandler/AC_MainWidgetHandler.AC_MainWidgetHandler_C"))
  (bind _wb_maingui (Variables|/Game/DialogueQuests/Blueprints/WidgetHandler/AC_MainWidgetHandler.AC_MainWidgetHandler_C|GetWB_MainGUI _returnvalue_2))
  (bind _wb_maingameplaymenu (Variables|/Game/DialogueQuests/UI/Widgets/Menu/WB_MainGUI.WB_MainGUI_C|GetWB_MainGameplayMenu _wb_maingui))
  (Utilities|IsValid _wb_maingui
    (:Is%20Valid
      (return (and (Widget|IsVisible _wb_maingameplaymenu) (== (Variables|/Game/DialogueQuests/UI/Widgets/MainGameplayGUI/WB_MainTopGUI.WB_MainTopGUI_C|GetCurrentMenuIndex (Variables|/Game/DialogueQuests/UI/Widgets/Menu/WB_MainGameplayMenu.WB_MainGameplayMenu_C|GetWB_MainTopGUI _wb_maingameplaymenu)) 6))))
    (:Is%20Not%20Valid
      (return false))))

(fn Equipable
  (params (Item :type S%20Items%20Inventory%20Structure))
  (return (Utilities|Enum|NotEqual(Enum) (.Subtype (Utilities|Struct|BreakS_ItemStatic (CallFunction|GetItemInfo (.Item (Utilities|Struct|BreakS_ItemsInventory Item))))) "NewEnumerator15")))

(fn GetWeightAngle
  (Utilities|IsValid (Variables|Default|GetPlayer)
    (:Is%20Valid
      (Variables|Default|SetCurrentWeight (Math|Float|Truncate (CallFunction|GetCurrentWeight)))
      (return (Math|Curves|GetFloatValue (Variables|Default|GetWalkSpeedCurve) (Math|Conversions|ToFloat(Integer) (- (Variables|Default|GetCurrentWeight) (CallFunction|GetMaxWeight))))))))

(fn FixItem
  (params (Index :type Integer) (Value :type Integer))
  (LocalVariables|SetL_Index Index)
  (LocalVariables|SetL_Value Value)
  (if (Utilities|Array|IsValidIndex (Variables|Inventory|GetInventory) (LocalVariables|GetL_Index))
    (Utilities|Array|SetArrayElem (Variables|Inventory|GetInventory) (LocalVariables|GetL_Index) (Utilities|Struct|MakeS_ItemsInventory (.Item (Utilities|Struct|BreakS_ItemsInventory (Utilities|Array|Get(acopy) (Variables|Inventory|GetInventory) (LocalVariables|GetL_Index)))) (.Amount (Utilities|Struct|BreakS_ItemsInventory (Utilities|Array|Get(acopy) (Variables|Inventory|GetInventory) (LocalVariables|GetL_Index)))) (.Modifications (Utilities|Struct|BreakS_ItemsInventory (Utilities|Array|Get(acopy) (Variables|Inventory|GetInventory) (LocalVariables|GetL_Index)))) (.SellerInformation (Utilities|Struct|BreakS_ItemsInventory (Utilities|Array|Get(acopy) (Variables|Inventory|GetInventory) (LocalVariables|GetL_Index)))) (Math|Integer|Clamp(Integer) (+ (.Qualoty (Utilities|Struct|BreakS_ItemsInventory (Utilities|Array|Get(acopy) (Variables|Inventory|GetInventory) (LocalVariables|GetL_Index)))) (LocalVariables|GetL_Value)) 0 100)))))

(fn GetActiveItematSlot
  (params (Type :type E_ItemSubtype%20Enum :default "NewEnumerator15")))

(fn UpdateFastItems)

(fn HandleFastItemInteract
  (params (Index :type Integer)))

(fn UseItem
  (params (Item :type S%20Items%20Inventory%20Structure%20%28by%20ref%29)))

(fn ApplyItemEffect
  (Utilities|IsValid (Actor|GetComponentbyClass (Components|GetOwner) 0)))

(fn CombineModificationArrays
  (params (Array :type Array%20of%20Data%20Table%20Row%20Handle%20Structures) (TargetArray :type Array%20of%20Data%20Table%20Row%20Handle%20Structures))
  (LocalVariables|SetL_ResArray Array)
  (for _array_element TargetArray
    (Utilities|Array|Add (LocalVariables|GetL_ResArray) _array_element))
  (return (LocalVariables|GetL_ResArray)))

(fn ApplyModifications
  (params (Item :type S%20Items%20Inventory%20Structure%20%28by%20ref%29)))

(fn DeapplyModification
  (params (Item :type S%20Items%20Inventory%20Structure)))

(fn MakePlayerViewSave)

(fn GetWeaponType)

(fn GetEfficiancy)

(fn AvailableLevel
  (params (Index :type Integer))
  (return (<= (.ReqLevel (Utilities|Struct|BreakS_ItemStatic (CallFunction|GetItemInfo (.Item (Utilities|Struct|BreakS_ItemsInventory (Utilities|Array|Get(acopy) (Variables|Inventory|GetInventory) Index)))))) (Variables|/Game/DialogueQuests/Blueprints/MapComponents/PlayerState/AC_ExpSystem.AC_ExpSystem_C|GetCurrentLevel (Actor|GetComponentbyClass (Components|GetOwner) "/Game/DialogueQuests/Blueprints/MapComponents/PlayerState/AC_ExpSystem.AC_ExpSystem_C")))))

(fn PlayItemSound
  (params (Index :type Integer))
  (Audio|PlaySoundatLocation (.Sound (Utilities|Struct|BreakS_ItemStatic (CallFunction|GetItemInfo (.Item (Utilities|Struct|BreakS_ItemsInventory (Utilities|Array|Get(acopy) (Variables|Inventory|GetInventory) Index)))))) (Transformation|GetActorLocation (Components|GetOwner))))

(fn GetMaxWeight
  (return (Variables|Default|GetMaxWeight)))

(fn InitialEquip)