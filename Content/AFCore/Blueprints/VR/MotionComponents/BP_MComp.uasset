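; Base actor for modular VR motion controller components, spawned under a parent BP_MotionController.
; On BeginPlay it waits in stages for controller, pawn and controller component to validate, registers with both controller and pawn, takes pawn ownership and caches side.
; It then runs setup, applies its active state and follows controller mesh visibility changes.
; Children override empty hooks for setup, visibility, key input and function input.
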(event Custom|SetupMComp
  ;[1 1 1] Overriden Initialize MComps
)

(event Custom|KeyPressed
  (params (Key :type Enum_Controller_Buttons%20Enum :default "NewEnumerator1") (Set :type Boolean))
  ;[1 1 1] Override KeyInput
)

(event Custom|FunctionInput
  (params (Function :type Name) (Set :type Boolean))
  ;[1 1 1] Override Function Input
)

(event Custom|MCompSetActive
  (params (Set :type Boolean))
  ;[1 1 1] Active Interface
  (Variables|State|SetActive Set))

(event Custom|MCompToggleActive
  ;[1 1 1] Active Interface
  (CallFunction|MCompSetActive (not (Variables|State|GetActive))))

(event Custom|MeshVisibilityChanged_Event_0
  (params (Set :type Boolean))
  ;[1 1 1] Setup
  (MComp|SetVisibility Set))

(event EventBeginPlay
  (bind _returnvalue (Actor|GetParentActor))
  ;[1 1 1] Setup
  (Utilities|WaitforObjecttoValidate _returnvalue 0.05
    (:Is%20Valid
      (bind _asbp_motion_controller (Utilities|Casting|CastToBP_MotionController _returnvalue))
      (bind _output_get (Variables|Setup|SetBaseMotionController _asbp_motion_controller))
      (Utilities|Map|Add (Variables|/Game/AFCore/Blueprints/VR/MotionControllers/BP_MotionController.BP_MotionController_C|GetMCompMap _asbp_motion_controller) (Utilities|GetClass self) self)
      (Utilities|WaitforObjecttoValidate (Variables|/Game/AFCore/Blueprints/VR/MotionControllers/BP_MotionController.BP_MotionController_C|GetVRPawn _output_get) 0.05
        (:Is%20Valid
          (Variables|Setup|SetVRPawn (Variables|/Game/AFCore/Blueprints/VR/MotionControllers/BP_MotionController.BP_MotionController_C|GetVRPawn _output_get))
          (Default|RegisterActortoPawn (Variables|/Game/AFCore/Blueprints/VR/MotionControllers/BP_MotionController.BP_MotionController_C|GetVRPawn _output_get) self true)
          (Actor|SetOwner (Variables|/Game/AFCore/Blueprints/VR/MotionControllers/BP_MotionController.BP_MotionController_C|GetVRPawn _output_get))
          (Utilities|WaitforObjecttoValidate (Variables|/Game/AFCore/Blueprints/VR/MotionControllers/BP_MotionController.BP_MotionController_C|GetMotionControllerComponent _output_get) 0.05
            (:Is%20Valid
              (Variables|Default|SetControllerComponent (Variables|/Game/AFCore/Blueprints/VR/MotionControllers/BP_MotionController.BP_MotionController_C|GetMotionControllerComponent _output_get))
              (Variables|Setup|SetSide (Variables|/Game/AFCore/Blueprints/VR/MotionControllers/BP_MotionController.BP_MotionController_C|GetSide _output_get))
              (CallFunction|SetupMComp)
              (CallFunction|MCompSetActive (Variables|State|GetActive))
              (EventDispatchers|AssignMeshVisibilityChanged (Variables|Setup|GetBaseMotionController) (delegate Custom|MeshVisibilityChanged_Event_0)))))))))

(event Collision|EventActorBeginOverlap
  (params (OtherActor :type Actor%20Object%20Reference)))

(fn ConstructionScript)

(fn SetVisibility
  (params (Set :type Boolean)))

(fn GetAllAttachedActors
  (return 0))