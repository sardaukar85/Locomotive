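; VR hand motion component that lets a player grab actors with Comp_Grab or latch onto Comp_Latch points.
; A timed sphere-trace from the hand highlights targets and triggers auto pickup, while Grab input grabs or releases.
; Grabs pull and attach or use a physics handle, latches snap the posed hand to sockets and auto-release out of range.
; Actions run locally first, then replicate via server multicast; held objects receive key and thumbstick input.
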(event BeforeDelete(Comp_Delete)
  (CallFunction|ExecuteReleaseActor))

(event Custom|Multi_LatchActor
  (params (LatchComponent :type Comp%20Latch%20Object%20Reference) (SnapSceneComponent :type Scene%20Component%20Object%20Reference) (SnapSocket :type Name))
  ;[0.6577 0 1] Server Latch
  (Utilities|LocallyControlled
    (:False
      (CallFunction|ExecuteLatchActor LatchComponent SnapSceneComponent SnapSocket))))

(event Custom|Multi_ReleaseActor
  ;[0.6577 0 1] Server Release Actor
  (Utilities|LocallyControlled
    (:False
      (CallFunction|ExecuteReleaseActor))))

(event Custom|PullActor
  (params (RelativeTransform :type Transform%20%28by%20ref%29) (KeepRotation :type Boolean))
  ;[0 0.566 1] Pull Grabbed Actor to correct Position on Hand
  (bind _out (CallFunction|SaveTransform (Transformation|GetActorTransform (Variables|Required|GetGrabbedActor))))
  (Components|Timeline|SetPlayRate (Variables|Default|GetPullTimeline) (Math|Float|MapRangeClamped (Math|Vector|Distance(Vector) (.Location (Math|Transform|BreakTransform _out)) (Math|Vector|SelectVector (- (Transformation|GetWorldLocation (Variables|Default|GetSecondHandle)) (.Location (Math|Transform|BreakTransform RelativeTransform))) (.Location (Math|Transform|BreakTransform (Transformation|GetWorldTransform (Variables|Default|GetSecondHandle)))) KeepRotation)) 2e+01 2e+03 3.0 0.4))
  (bind _procent (Timeline|PullTimeline PlayFromStart)
    (:Update
      (if KeepRotation
        (Transformation|SetActorLocation (Variables|Required|GetGrabbedActor) (Math|Vector|Lerp(Vector) (.Location (Math|Transform|BreakTransform _out)) (- (Transformation|GetWorldLocation (Variables|Default|GetSecondHandle)) (.Location (Math|Transform|BreakTransform RelativeTransform))) _procent) false false)
        (else
          (Transformation|SetActorTransform (Variables|Required|GetGrabbedActor) (Math|Transform|Lerp(Transform) _out (Transformation|GetWorldTransform (Variables|Default|GetSecondHandle)) _procent) false true))))
    (:Finished
      (Utilities|IsValid (Actor|GetAttachParentActor (Variables|Required|GetGrabbedActor))
        (:Is%20Not%20Valid
          (|PlayGrabbedSound))))))

(event Custom|LatchActor
  (params (LatchComponent :type Comp%20Latch%20Object%20Reference) (SnapSceneComponent :type Scene%20Component%20Object%20Reference) (SnapSocket :type Name))
  ;[1 1 1] Latch
  (CallFunction|ExecuteLatchActor LatchComponent SnapSceneComponent SnapSocket)
  (Utilities|DoesActorOfComponentReplicate LatchComponent
    (:True
      (CallFunction|ServerLatchActor LatchComponent SnapSceneComponent SnapSocket))))

(event Custom|ExecuteLatchActor
  (params (LatchComponent :type Comp%20Latch%20Object%20Reference) (SnapSceneComponent :type Scene%20Component%20Object%20Reference) (SnapSocket :type Name))
  ;[0 0.566 1] Multicast Latch
  (bind _output_get (Variables|Default|SetLatchComponent LatchComponent))
  (Variables|Required|SetGrabbedActor (Components|GetOwner _output_get))
  (Default|SnaptoSocket (Variables|Required|GetMotionControllerHands) SnapSceneComponent SnapSocket)
  (Default|SetPose (Variables|Required|GetMotionControllerHands) true (Utilities|SocketNametoPose SnapSocket))
  (Variables|Required|SetLatch true)
  (Utilities|LocallyControlled
    (:True
      (Default|CreateLatchingHelper (Variables|Default|GetLatchComponent) (Transformation|GetSocketTransform (Variables|/Game/AFCore/Blueprints/VR/MotionControllers/BP_MotionController_Hands.BP_MotionController_Hands_C|GetHandMesh (Variables|Required|GetMotionControllerHands)) "GrabSearch" "RTS_World") self (Variables|Default|GetDefaultSceneRoot))
      (EventDispatchers|BindEventtoAutoReleaseReached (delegate Custom|AutoReleaseReached_Event)))
    (:False
      _))
  (Default|LatchPressed (Variables|Default|GetLatchComponent) (Variables|Default|GetVRPawn) self)
  (Utilities|SetHandCollision "NoCollision"))

(event Custom|GrabActor
  (params (Actor :type Actor%20Object%20Reference) (DesiredRelativeTransform :type Transform) (KeepRotation :type Boolean) (GrabPose :type Enum_Grab_Pose%20Enum :default "NewEnumerator0") (SnapSceneComponent :type Scene%20Component%20Object%20Reference) (SnapSocket :type Name))
  ;[1 1 1] Grab
  (CallFunction|ExecuteGrabActor Actor DesiredRelativeTransform KeepRotation GrabPose SnapSceneComponent SnapSocket)
  (Utilities|DoesActorReplicate Actor
    (:True
      (CallFunction|ServerGrabActor Actor DesiredRelativeTransform KeepRotation GrabPose SnapSceneComponent SnapSocket))))

(event Custom|Execute_GrabActor
  (params (Actor :type Actor%20Object%20Reference) (DesiredActorTransform :type Transform) (KeepRotation :type Boolean) (GrabPose :type Enum_Grab_Pose%20Enum :default "NewEnumerator0") (SnapSceneComponent :type Scene%20Component%20Object%20Reference) (SnapSocket :type Name))
  ;[0 0.566 1] Multicast Grab
  (Variables|Required|SetGrabbedActor Actor)
  (Variables|Required|SetLatch false)
  (CallFunction|DetachActorfromEverything (Variables|Required|GetGrabbedActor))
  (Default|SetPose (Variables|Required|GetMotionControllerHands) true GrabPose)
  (|PickUpHaptics)
  (switch Utilities|FlowControl|Switch|SwitchonEnum_Grab_Type (Variables|/Game/AFCore/Blueprints/Components/Interaction/Comp_Grab.Comp_Grab_C|GetGrabType (Actor|GetComponentbyClass (Variables|Required|GetGrabbedActor) "/Game/AFCore/Blueprints/Components/Interaction/Comp_Grab.Comp_Grab_C"))
    (:NewEnumerator0
      (|RelocateHandlesAndPull DesiredActorTransform KeepRotation)
      (Transformation|AttachComponentToComponent (Variables|Required|GetGrabbedActor) (Variables|Default|GetSecondHandle) "AttachPoint" "KeepWorld" "KeepWorld" "KeepWorld" true))
    (:NewEnumerator1
      (Utilities|IsValid SnapSceneComponent
        (:Is%20Valid
          (Physics|Components|PhysicsHandle|GrabComponentatLocationwithRotation (Variables|Default|GetPhysicsHandle) (.AsPrimitive%20Component (Utilities|Casting|CastToPrimitiveComponent SnapSceneComponent)) "None" (Transformation|GetSocketLocation SnapSceneComponent SnapSocket) (Transformation|GetSocketRotation SnapSceneComponent SnapSocket))
          (Default|SnaptoSocket (Variables|Required|GetMotionControllerHands) SnapSceneComponent SnapSocket))
        (:Is%20Not%20Valid
          (Physics|Components|PhysicsHandle|GrabComponentatLocationwithRotation (Variables|Default|GetPhysicsHandle) (.AsPrimitive%20Component (Utilities|Casting|CastToPrimitiveComponent (Variables|/Script/Engine.Actor|GetRootComponent (Variables|Required|GetGrabbedActor)))) "None" (+ (Transformation|GetActorLocation (Variables|Required|GetGrabbedActor)) (.Location (Math|Transform|BreakTransform DesiredActorTransform))) (Transformation|GetActorRotation (Variables|Required|GetGrabbedActor)))))
      (Utilities|SetHandCollision "NoCollision")))
  (Default|GrabPressed (Actor|GetComponentbyClass (Variables|Required|GetGrabbedActor) "/Game/AFCore/Blueprints/Components/Interaction/Comp_Grab.Comp_Grab_C") (Variables|Default|GetVRPawn) self)
  (if (Variables|/Game/AFCore/Blueprints/Components/Interaction/Comp_Grab.Comp_Grab_C|GetSnapAndReplaceControls (Actor|GetComponentbyClass (Variables|Required|GetGrabbedActor) "/Game/AFCore/Blueprints/Components/Interaction/Comp_Grab.Comp_Grab_C"))
    (Default|SetReplacedControls (Variables|Default|GetBaseMotionController) self (Utilities|Struct|MakeStruct_MotionController_Occupied true (Utilities|Array|MakeArray) (Utilities|Array|MakeArray)))))

(event Custom|Server_ReleaseActor
  ;[0.6577 0 1] Server Release Actor
  (CallFunction|MultiReleaseActor))

(event Custom|ExecuteReleaseActor
  ;[0 0.566 1] Multicast Actor Released
  (Default|SetPose (Variables|Required|GetMotionControllerHands) false "NewEnumerator0")
  (Default|SnaptoSocket (Variables|Required|GetMotionControllerHands) 0 "None")
  (|ReleaseHaptics)
  (if (Variables|Required|GetLatch)
    (Variables|Required|SetGrabbedActor 0)
    (EventDispatchers|UnbindallEventsfromAutoReleaseReached)
    (bind _latchcomponent (Variables|Default|GetLatchComponent)
      (:then
        (Default|LatchReleased _latchcomponent self)
        (Variables|Default|SetLatchComponent 0))
      (:else))
    (else
      (Variables|Required|GetGrabbedActor
        (:then
          (|PlayReleasedSound)
          (CallFunction|StopPull)
          (Transformation|DetachFromActor (Variables|Required|GetGrabbedActor) "KeepWorld" "KeepWorld" "KeepWorld")
          (|ResetSnapControls (Actor|GetComponentbyClass (Variables|Required|GetGrabbedActor) "/Game/AFCore/Blueprints/Components/Interaction/Comp_Grab.Comp_Grab_C"))
          (Default|GrabReleased (Actor|GetComponentbyClass (Variables|Required|GetGrabbedActor) "/Game/AFCore/Blueprints/Components/Interaction/Comp_Grab.Comp_Grab_C") self)
          (Variables|Required|SetGrabbedActor 0)
          (Physics|Components|PhysicsHandle|ReleaseComponent (Variables|Default|GetPhysicsHandle)))
        (:else))))
  (Utilities|SetHandCollision "NoCollision")
  (Utilities|FlowControl|Delay 2.0)
  (Variables|Required|GetGrabbedActor
    (:then)
    (:else
      (Utilities|SetHandCollision "QueryAndPhysics"))))

(event Custom|Server_LatchActor
  (params (LatchComponent :type Comp%20Latch%20Object%20Reference) (SnapSceneComponent :type Scene%20Component%20Object%20Reference) (SnapSocket :type Name))
  ;[0.6577 0 1] Server Latch
  (CallFunction|MultiLatchActor LatchComponent SnapSceneComponent SnapSocket))

(event Custom|StopPull
  ;[0 0.566 1] Pull Grabbed Actor to correct Position on Hand
  (bind _procent (Timeline|PullTimeline Stop)
    (:Update
      (if (stale Custom|PullActor KeepRotation)
        (Transformation|SetActorLocation (Variables|Required|GetGrabbedActor) (Math|Vector|Lerp(Vector) (.Location (Math|Transform|BreakTransform (stale Custom|PullActor _out))) (- (Transformation|GetWorldLocation (Variables|Default|GetSecondHandle)) (.Location (Math|Transform|BreakTransform (stale Custom|PullActor RelativeTransform)))) _procent) false false)
        (else
          (Transformation|SetActorTransform (Variables|Required|GetGrabbedActor) (Math|Transform|Lerp(Transform) (stale Custom|PullActor _out) (Transformation|GetWorldTransform (Variables|Default|GetSecondHandle)) _procent) false true))))
    (:Finished
      (Utilities|IsValid (Actor|GetAttachParentActor (Variables|Required|GetGrabbedActor))
        (:Is%20Not%20Valid
          (|PlayGrabbedSound))))))

(event Custom|SetSearchTickForPickup
  (params (Condition :type Boolean))
  ;[1 1 1] Search For Objects to Highlight and Auto Pickup
  (Utilities|WhileLoopwithDelay Condition (Variables|Internal|GetSearchTickTime)
    (:LoopBody
      (Utilities|IsGrabbingActor
        (:false
          (|IsHandOpen
            (:OutputPin
              (|SearchforPickup))))))))

(event Custom|Multi_GrabActor
  (params (Actor :type Actor%20Object%20Reference) (DesiredActorTransform :type Transform) (KeepRotation :type Boolean) (GrabPose :type Enum_Grab_Pose%20Enum :default "NewEnumerator0") (SnapSceneComponent :type Scene%20Component%20Object%20Reference) (SnapSocket :type Name))
  ;[0.6577 0 1] Server Grab
  (Utilities|LocallyControlled
    (:False
      (CallFunction|ExecuteGrabActor Actor DesiredActorTransform KeepRotation GrabPose SnapSceneComponent SnapSocket))))

(event Custom|Server_GrabActor
  (params (Actor :type Actor%20Object%20Reference) (DesiredRelativeTransform :type Transform) (KeepRotation :type Boolean) (GrabPose :type Enum_Grab_Pose%20Enum :default "NewEnumerator0") (SnapSceneComponent :type Scene%20Component%20Object%20Reference) (SnapSocket :type Name))
  ;[0.6577 0 1] Server Grab
  (CallFunction|MultiGrabActor Actor DesiredRelativeTransform KeepRotation GrabPose SnapSceneComponent SnapSocket))

(event Custom|AutoReleaseReached_Event
  ;[0 0.566 1] Multicast Latch
  (EventDispatchers|UnbindEventfromAutoReleaseReached (delegate Custom|AutoReleaseReached_Event))
  (CallFunction|GrabbingActorReleaseActor))

(event EventBeginPlay
  (bind _returnvalue (Actor|GetParentActor))
  (|CallParentFunction)
  (Utilities|WaitforObjecttoValidate _returnvalue 0.05
    (:Is%20Valid
      (bind _asbp_motion_controller_hands (Utilities|Casting|CastToBP_MotionController_Hands _returnvalue))
      (Variables|Required|SetMotionControllerHands _asbp_motion_controller_hands)
      (CallFunction|SetSearchTickforPickup true))))

(event EventTick
  (params (DeltaSeconds :type Float%20%28single-precision%29))
  (|CallParentFunction DeltaSeconds)
  (Utilities|LocallyControlled
    (:True
      (Utilities|IsGrabbingActor
        (:true
          ;[1 1 1] Forward Thumbstick Input if Object is Grabbed
          (|ForwardThumbstickToHeldObject)
          (|AutoReleaseLatch)
          (Class|PhysicsHandleComponent|SetTargetLocationandRotation (Variables|Default|GetPhysicsHandle) (Transformation|GetActorLocation) (Transformation|GetActorRotation)))))))

(event EventGrabbingActorReleaseActor
  ;[1 1 1] Release Actor
  (CallFunction|ExecuteReleaseActor)
  (CallFunction|ServerReleaseActor))

(event EventDebugSetDebugGrab
  (params (Set :type Boolean))
  ;[1 1 1] Debug Mode
  (Variables|Debug|SetDebug_TraceGrab Set))

(event EventGrabbingActorGrabActor
  (params (PreferedActor :type Actor%20Object%20Reference) (GrabComponent :type Comp%20Grab%20Object%20Reference) (LatchComponent :type Comp%20Latch%20Object%20Reference))
  ;[1 1 1] Try to Latch Or Grab
  (Interaction|CheckforGraborLatch PreferedActor))

(event EventKeyPressed
  (params (Key :type Enum_Controller_Buttons%20Enum :default "NewEnumerator1") (Set :type Boolean))
  (bind _grabbedactor (Variables|Required|GetGrabbedActor))
  (bind _returnvalue (Actor|GetComponentbyClass _grabbedactor "/Game/AFCore/Blueprints/Components/Interaction/Comp_Grab.Comp_Grab_C"))
  ;[1 1 1] Forward KeyInputs to Grabbed Object
  (|CallParentFunction Key Set)
  (Utilities|IsValid _grabbedactor
    (:Is%20Valid
      (Utilities|IsValid _returnvalue
        (:Is%20Valid
          (Default|KeyPressed _returnvalue Key Set))))))

(event EventFunctionInput
  (params (Function :type Name :default "None") (Set :type Boolean))
  (bind _vrpawn (Variables|Default|GetVRPawn))
  (bind _controlcomponent (Default|GetControlComponent _vrpawn))
  (bind _holdinggrip (Default|GetHoldingGrip _controlcomponent))
  ;[1 1 1] KeyInputs
  (|CallParentFunction Function Set)
  (switch name Function
    (:Grab
      ;[1 1 1] Handle Grab
      (if Set
        (if _holdinggrip
          (Utilities|IsValid (Variables|Required|GetGrabbedActor)
            (:Is%20Not%20Valid
              (CallFunction|GrabbingActorGrabActor :!label _label)))
          (else
            (Utilities|IsValid (Variables|Required|GetGrabbedActor)
              (:Is%20Valid
                (CallFunction|GrabbingActorReleaseActor))
              (:Is%20Not%20Valid
                (goto _label)))))
        (elif _holdinggrip
          (Utilities|IsValid (Variables|Required|GetGrabbedActor)
            (:Is%20Valid
              (CallFunction|GrabbingActorReleaseActor))))))))

(fn ConstructionScript)

(fn CheckforGraborLatch
  (params (PreferredTarget :type Actor%20Object%20Reference))
  (Utilities|IsValid PreferredTarget
    (:Is%20Valid
      (bind (_canbegrabbed _actortouse _latch _latchcomponent _grabcomponent) (Interaction|CheckifActorCanbeGrabbed PreferredTarget 0 (Transformation|GetActorLocation)))
      (if _canbegrabbed
        (|SetLocalVariables_2 _actortouse (Transformation|GetActorLocation _actortouse) _latchcomponent _grabcomponent)
        (if _latch
          (bind (_scenecomponent _socketname) (Default|GetClosestAttachPoint (LocalVariables|GetLocalLatchComponent) (Transformation|GetSocketLocation (Variables|/Game/AFCore/Blueprints/VR/MotionControllers/BP_MotionController_Hands.BP_MotionController_Hands_C|GetHandMesh (Variables|Required|GetMotionControllerHands)) "GrabSearch") (Utilities|Select :Index (Variables|Default|GetSide) :NewEnumerator0 "L_" :NewEnumerator1 "R_") true 2.0 :!label _label))
          (CallFunction|LatchActor (LocalVariables|GetLocalLatchComponent) _scenecomponent _socketname)
          (else
            (bind (_scenecomponent_2 _socketname_2) (Default|GetClosestHandSocket (LocalVariables|GetLocalGrabComponent) (LocalVariables|GetLocalImpactLocation) (Variables|Default|GetSide) :!label _label_2))
            (Utilities|IsValid _scenecomponent_2
              (:Is%20Valid
                (CallFunction|GrabActor (LocalVariables|GetLocalActorToUse) (|InvertOnLeftHand (Transformation|GetSocketTransform _scenecomponent_2 _socketname_2 "RTS_Actor")) false (Utilities|Enum|ByteToEnumEnum_Grab_Pose (Math|Conversions|ToByte(Integer) (Math|Conversions|ToInteger(Byte) (Utilities|String|GetSubstring (Utilities|String|ToString(Name) _socketname_2) 2 2)))) _scenecomponent_2 _socketname_2))
              (:Is%20Not%20Valid
                (CallFunction|GrabActor (LocalVariables|GetLocalActorToUse) (Math|Transform|MakeTransform (- (+ (LocalVariables|GetLocalImpactLocation) (- (Transformation|GetActorLocation) (Transformation|GetWorldLocation (Variables|Default|GetGrabOffset)))) (Transformation|GetActorLocation (LocalVariables|GetLocalActorToUse)))) true "NewEnumerator0" 0 "None")))))))
    (:Is%20Not%20Valid
      (bind (_location _impactnormal _hitactor _hitcomponent) (Utilities|Trace)
        (:then
          (bind (_canbegrabbed_2 _actortouse_2 _latch_2 _latchcomponent_2 _grabcomponent_2) (Interaction|CheckifActorCanbeGrabbed _hitactor _hitcomponent _location))
          (if _canbegrabbed_2
            (|SetLocalVariables _actortouse_2 _location _latchcomponent_2 _grabcomponent_2)
            (if _latch_2
              (goto _label)
              (else
                (goto _label_2)))))))))

(fn GetAllAttachedActors
  (bind _actors (|CallParentFunction))
  (LocalVariables|SetReturn _actors)
  (Utilities|Set|Add (LocalVariables|GetReturn) (Variables|Required|GetGrabbedActor))
  (return (LocalVariables|GetReturn)))

(fn CheckifActorCanbeGrabbed
  (params (ActorToGrab :type Actor%20Object%20Reference) (HitComponent :type Primitive%20Component%20Object%20Reference) (ReferencingLocation :type Vector))
  (bind _returnvalue (Actor|GetComponentbyClass ActorToGrab "/Game/AFCore/Blueprints/Components/Interaction/Comp_Grab.Comp_Grab_C"))
  (bind _self self)
  (bind _grabidentifier (Variables|Grab|GetGrabIdentifier))
  (bind _vrpawn (Variables|Default|GetVRPawn))
  (bind _struct_component_sourceinfo (Utilities|Struct|MakeStruct_Component_SourceInfo _vrpawn ReferencingLocation _self _self _grabidentifier))
  (for _array_element (Actor|GetComponentsByClass ActorToGrab "/Game/AFCore/Blueprints/Components/Interaction/Comp_Latch.Comp_Latch_C")
    (bind _latchable (Default|CanbeLatchedonTo? _array_element (Transformation|GetSocketLocation (Variables|/Game/AFCore/Blueprints/VR/MotionControllers/BP_MotionController_Hands.BP_MotionController_Hands_C|GetHandMesh (Variables|Required|GetMotionControllerHands)) "GrabSearch") (Utilities|Array|MakeArray "NewEnumerator3" "NewEnumerator0" "NewEnumerator1" "NewEnumerator2" "NewEnumerator4") "AttachPoint" _struct_component_sourceinfo))
    (if _latchable
      (return true ActorToGrab true _array_element 0)))
  (Utilities|IsValid _returnvalue
    (:Is%20Valid
      (bind _isgrabbable (Default|CanbeGrabbed _returnvalue HitComponent _struct_component_sourceinfo))
      (if _isgrabbable
        (bind _returnvalue_2 (Default|GetActortobeGrabbed _returnvalue))
        (return true _returnvalue_2 false 0 (Actor|GetComponentbyClass _returnvalue_2 "/Game/AFCore/Blueprints/Components/Interaction/Comp_Grab.Comp_Grab_C"))
        (else
          _)))
    (:Is%20Not%20Valid
      _))
  (return false 0 false 0 0))

(fn DebugGetGazeInfo
  (return ""))

(fn DebugGetGrabInfo
  (bind _debug_tracedgrabbedactor (Variables|Debug|GetDebug_TracedGrabbedActor))
  (Utilities|IsValid _debug_tracedgrabbedactor
    (:Is%20Valid
      (return (Utilities|Text|FormatText "{Side} Grab: {Actor}" (Utilities|String|EnumtoString (Variables|Default|GetSide)) (Utilities|GetDisplayName _debug_tracedgrabbedactor))))
    (:Is%20Not%20Valid
      (return ""))))

(fn DebugGetSelectInfo
  (return ""))

(fn GrabbingActorGetCurrentlyGrabbedActor
  (return (Variables|Required|GetGrabbedActor)))

(fn GrabbingActorSupportPhysicsHandle
  (return true))