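; BP_Manager_Spectator is a manager that tracks spectator components by key and controls which one feeds the VR spectator screen.
; Activating a spectator stops the previous one's capture, starts the new one, broadcasts its owner and render target, and reapplies the preferred screen mode.
; Screen modes show the texture fullscreen or combine it with the eye view as a top-right inset either way.
; Deactivation restores the cropped single-eye view.
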(event Custom|RegisterSpectator
  (params (SpectatorComponent :type Comp%20Spectator%20Object%20Reference%20%28by%20ref%29) (Key :type Name%20%28by%20ref%29))
  (if (Utilities|Name|NotEqual(Name) Key "None")
    (Utilities|Map|Add (Variables|Default|GetSpectatorMap) Key SpectatorComponent)
    (else
      (Development|PrintString (Utilities|String|Append "Can't register spectator " (Utilities|GetDisplayName SpectatorComponent) " because key is not set")))))

(event Custom|ActivateSpectator
  (params (Spectator :type Comp%20Spectator%20Object%20Reference))
  (if (!= Spectator (Variables|Default|GetCurrentlyActiveSpectator))
    (CallFunction|DeactivateActiveSpectator)
    (Variables|Default|SetCurrentlyActiveSpectator Spectator)
    (Default|StartCapture Spectator)
    (Default|CallNewSpectatorActivated Spectator (Components|GetOwner Spectator) (Default|GetRenderTarget Spectator))
    (CallFunction|SetScreenMode (Variables|Default|GetPreferredScreenMode))))

(event Custom|DeactivateActiveSpectator
  (bind _currentlyactivespectator (Variables|Default|GetCurrentlyActiveSpectator)
    (:then
      (CallFunction|DeactivateSpectator _currentlyactivespectator))
    (:else)))

(event Custom|ActivateSpecatorByKey
  (params (Key :type Name%20%28by%20ref%29))
  (bind _spectatormap (Variables|Default|GetSpectatorMap))
  (bind (_value _returnvalue) (Utilities|Map|Find _spectatormap Key))
  (if _returnvalue
    (CallFunction|ActivateSpectator _value)))

(event Custom|SetScreenMode
  (params (ScreenMode :type Enum_Spectator_Modes%20Enum :default "NewEnumerator0"))
  (bind _output_get (Variables|Default|SetPreferredScreenMode ScreenMode))
  (switch Utilities|FlowControl|Switch|SwitchonEnum_Spectator_Modes _output_get
    (:NewEnumerator0
      (Class|HeadMountedDisplayFunctionLibrary|SetSpectatorScreenMode "Texture"))
    (:NewEnumerator1
      (Class|HeadMountedDisplayFunctionLibrary|SetSpectatorScreenMode "TexturePlusEye")
      (Class|HeadMountedDisplayFunctionLibrary|SetSpectatorScreenModeTexturePlusEyeLayout "(X=0.700000,Y=0.020000)" "(X=0.980000,Y=0.400000)" "(X=0.000000,Y=0.000000)" "(X=1.000000,Y=1.000000)" false false false))
    (:NewEnumerator2
      (Class|HeadMountedDisplayFunctionLibrary|SetSpectatorScreenMode "TexturePlusEye")
      (Class|HeadMountedDisplayFunctionLibrary|SetSpectatorScreenModeTexturePlusEyeLayout "(X=0.000000,Y=0.000000)" "(X=1.000000,Y=1.000000)" "(X=0.700000,Y=0.020000)" "(X=0.980000,Y=0.400000)" true false false))))

(event Custom|DeactivateSpectator
  (params (Spectator :type Comp%20Spectator%20Object%20Reference))
  (if (== Spectator (Variables|Default|GetCurrentlyActiveSpectator))
    (Variables|Default|SetCurrentlyActiveSpectator 0)
    (Default|StopCapture Spectator)
    (Class|HeadMountedDisplayFunctionLibrary|SetSpectatorScreenMode "SingleEyeCroppedToFill")))

(fn ConstructionScript)