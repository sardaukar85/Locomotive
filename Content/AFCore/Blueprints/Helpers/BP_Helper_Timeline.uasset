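; Helper actor that runs a keyed timeline over a configurable duration, forward or in reverse, for other logic to receive progress.
; BeginPlay scales the play rate by the inverse of Duration and starts playback, or sends full progress immediately when Duration is not positive.
; Updates broadcast the Key with progress from the selected linear or easing curve.
; Finishing broadcasts the end event and destroys the actor; Play and Stop control playback.
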(event Custom|Play
  (params (Direction :type Boolean))
  (bind _output_get (Variables|Default|SetDirection Direction))
  (if _output_get
    (bind (_direction _easeinandout _linear _easein _easeout) (Timeline|MainTimeline Play)
      (:Update
        (Default|CallUpdateProgress (Variables|Default|GetKey) (Utilities|Select :Index (Variables|Default|GetCurve) :NewEnumerator0 _easeinandout :NewEnumerator1 _linear :NewEnumerator2 _easein :NewEnumerator3 _easeout)))
      (:Finished
        (Default|CallTimelineEnded (Variables|Default|GetKey))
        (Actor|DestroyActor)))
    (else
      (Timeline|MainTimeline Reverse))))

(event Custom|Stop
  (bind (_direction _easeinandout _linear _easein _easeout) (Timeline|MainTimeline Stop)
    (:Update
      (Default|CallUpdateProgress (Variables|Default|GetKey) (Utilities|Select :Index (Variables|Default|GetCurve) :NewEnumerator0 _easeinandout :NewEnumerator1 _linear :NewEnumerator2 _easein :NewEnumerator3 _easeout)))
    (:Finished
      (Default|CallTimelineEnded (Variables|Default|GetKey))
      (Actor|DestroyActor))))

(event EventBeginPlay
  (if (> (Variables|Default|GetDuration) 0.0)
    (Components|Timeline|SetPlayRate (Variables|Default|GetMainTimeline) (/ 1.0 (Variables|Default|GetDuration)))
    (if (Variables|Default|GetDirection)
      (bind (_direction _easeinandout _linear _easein _easeout) (Timeline|MainTimeline PlayFromStart)
        (:Update
          (Default|CallUpdateProgress (Variables|Default|GetKey) (Utilities|Select :Index (Variables|Default|GetCurve) :NewEnumerator0 _easeinandout :NewEnumerator1 _linear :NewEnumerator2 _easein :NewEnumerator3 _easeout)))
        (:Finished
          (Default|CallTimelineEnded (Variables|Default|GetKey))
          (Actor|DestroyActor)))
      (else
        (Timeline|MainTimeline ReverseFromEnd)))
    (else
      (Default|CallUpdateProgress (Variables|Default|GetKey) 1.0))))

(event Collision|EventActorBeginOverlap
  (params (OtherActor :type Actor%20Object%20Reference)))

(event EventTick
  (params (DeltaSeconds :type Float%20%28single-precision%29)))

(fn ConstructionScript)