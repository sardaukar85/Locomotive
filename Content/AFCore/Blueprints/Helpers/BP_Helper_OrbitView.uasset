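; BP_Helper_OrbitView is an orbit camera helper with a Camera and SpringArm that offers look, zoom and camera position functions.
; Look events rotate the arm in pitch and yaw, Zoom changes its length, and construction sets the initial distance.
; Tick softly eases arm length and pitch back into their allowed ranges instead of hard clamping.
; A timeline event blends the camera's relative transform from its saved value back to identity.
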(event Custom|Zoom
  (params (Factor :type Float%20%28single-precision%29))
  (Variables|/Script/Engine.SpringArmComponent|SetTargetArmLength (Variables|Default|GetSpringArm) (+ Factor (Variables|/Script/Engine.SpringArmComponent|GetTargetArmLength (Variables|Default|GetSpringArm)))))

(event Custom|CustomEvent_0
  (bind _out (CallFunction|SaveTransform (Transformation|GetRelativeTransform (Variables|Default|GetCamera))))
  (bind _percent (Timeline|RepositionCameraTimeline PlayFromStart)
    (:Update
      (Transformation|SetRelativeTransform (Variables|Default|GetCamera) (Math|Transform|Lerp(Transform) _out (Math|Transform|MakeTransform "0, 0, 0" "0, 0, 0" "1,1,1") _percent) false false))))

(event Custom|LookUp
  (params (AxisValue :type Float%20%28single-precision%29))
  (Transformation|AddRelativeRotation (Variables|Default|GetSpringArm) (Math|Rotator|MakeRotator 0.0 AxisValue 0.0) false false))

(event Custom|LookRight
  (params (AxisValue :type Float%20%28single-precision%29))
  (Transformation|AddRelativeRotation (Variables|Default|GetSpringArm) (Math|Rotator|MakeRotator 0.0 0.0 AxisValue) false false))

(event EventBeginPlay)

(event Collision|EventActorBeginOverlap
  (params (OtherActor :type Actor%20Object%20Reference)))

(event EventTick
  (params (DeltaSeconds :type Float%20%28single-precision%29))
  (bind _springarm (Variables|Default|GetSpringArm))
  (bind _zoomrange (Variables|Default|GetZoomRange))
  (bind _pitchrange (Variables|Default|GetPitchRange))
  (bind _relativerotation (Variables|/Script/Engine.SceneComponent|GetRelativeRotation _springarm))
  (Utilities|FlowControl|Sequence
    (:then_0
      (if (not (Math|Float|InRange(Float) (Variables|/Script/Engine.SpringArmComponent|GetTargetArmLength (Variables|Default|GetSpringArm)) (.min _zoomrange) (.max _zoomrange) false false))
        (Variables|/Script/Engine.SpringArmComponent|SetTargetArmLength (Variables|Default|GetSpringArm) (Math|Interpolation|FInterpTo (Variables|/Script/Engine.SpringArmComponent|GetTargetArmLength (Variables|Default|GetSpringArm)) (select (< (Variables|/Script/Engine.SpringArmComponent|GetTargetArmLength (Variables|Default|GetSpringArm)) (.max _zoomrange)) (.min _zoomrange) (.max _zoomrange)) DeltaSeconds 2.0))))
    (:then_1
      (if (not (Math|Float|InRange(Float) (.pitch _relativerotation) (.min _pitchrange) (.max _pitchrange) false false))
        (Transformation|AddRelativeRotation (Variables|Default|GetSpringArm) (Math|Rotator|MakeRotator 0.0 (/ (select (< (.pitch _relativerotation) (.max _pitchrange)) (- (.min _pitchrange) (.pitch _relativerotation)) (- (.max _pitchrange) (.pitch _relativerotation))) 5.0) 0.0) false false)))))

(fn ConstructionScript
  (Variables|/Script/Engine.SpringArmComponent|SetTargetArmLength (Variables|Default|GetSpringArm) (Variables|Default|GetInitialDistance)))

(fn GetCameraPosition
  (bind _camera (Variables|Default|GetCamera))
  (return (Transformation|GetWorldLocation _camera) (Transformation|GetWorldRotation _camera)))