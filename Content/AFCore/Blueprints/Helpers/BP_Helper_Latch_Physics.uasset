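; Latch helper Blueprint that adds physics-constraint attachment to its parent's latch behavior.
; When latched, it constrains its Handle to the attached component at the attached socket and listens for the constraint breaking.
; A broken constraint messages the latching actor to release its grab.
; On latch release, it breaks the constraint and then unbinds that listener.
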(event Custom|OnConstraintBroken_Event_0
  (params (ConstraintIndex :type Integer))
  (Class|InterfaceGrabbingActor|GrabbingActorReleaseActor(Message) (stale EventActorGotLatched LatchingActor)))

(event EventActorGotLatched
  (params (LatchingPawn :type BP%20Pawn%20Base%20Object%20Reference) (LatchingActor :type Actor%20Object%20Reference))
  (|CallParentFunction LatchingPawn LatchingActor)
  (Class|PhysicsConstraintComponent|SetConstrainedComponents (Variables|Default|GetPhysicsConstraint) (Variables|Default|GetHandle) "None" (.AsPrimitive%20Component (Utilities|Casting|CastToPrimitiveComponent (Variables|Default|GetAttachedComponent))) (Variables|Default|GetAttachedSocket))
  (EventDispatchers|AssignOnConstraintBroken (Variables|Default|GetPhysicsConstraint) (delegate Custom|OnConstraintBroken_Event_0)))

(event EventActorLatchReleased
  (params (ReleasingPawn :type BP%20Pawn%20Base%20Object%20Reference) (ReleasingActor :type Actor%20Object%20Reference))
  (|CallParentFunction ReleasingPawn ReleasingActor)
  (Class|PhysicsConstraintComponent|BreakConstraint (Variables|Default|GetPhysicsConstraint))
  (EventDispatchers|UnbindEventfromOnConstraintBroken (Variables|Default|GetPhysicsConstraint) (delegate Custom|OnConstraintBroken_Event_0)))

(fn ConstructionScript
  (|CallParentFunction))

(fn Get
  (return 0))