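; Temporary helper pawn that hands a joining player over to their real pawn spawn, then destroys itself when unpossessed.
; On authority, a gate waits until both BeginPlay and Possessed have fired, while remote instances proceed directly from BeginPlay.
; If locally controlled, it blacks out the camera and calls ServerSpawnPawn, which gets a player index from BP_GameMode_Main and passes it with level info to the controller's ClientSpawnPawn.
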(event Custom|ServerSpawnPawn
  (params (Controller :type Controller%20Object%20Reference))
  (bind _asbp_game_mode_main (Utilities|Casting|CastToBP_GameMode_Main (Game|GetGameMode)))
  (bind _asbp_player_controller_main (Utilities|Casting|CastToBP_PlayerController_Main Controller))
  (bind _newindex (Default|CreatePlayerIndex _asbp_game_mode_main _asbp_player_controller_main))
  (Default|ClientSpawnPawn _asbp_player_controller_main _newindex (CallFunction|GetInfoLevels self)))

(event EventBeginPlay
  (bind _returnvalue (Pawn|GetController))
  (Networking|SwitchHasAuthority
    (:Authority
      (Utilities|FlowControl|Sequence
        (:then_0
          (Utilities|FlowControl|Gate true :!label _label
            (:Exit
              _)))
        (:then_1
          (goto _label Open))))
    (:Remote
      _))
  (if (Pawn|IsLocallyControlled)
    (|CameraFade _returnvalue)
    (CallFunction|ServerSpawnPawn _returnvalue)))

(event Collision|EventActorBeginOverlap
  (params (OtherActor :type Actor%20Object%20Reference)))

(event EventTick
  (params (DeltaSeconds :type Float%20%28single-precision%29)))

(event EventPossessed
  (params (NewController :type Controller%20Object%20Reference))
  (bind _returnvalue (Pawn|GetController))
  (Networking|SwitchHasAuthority
    (:Authority
      (Utilities|FlowControl|Sequence
        (:then_0
          (Utilities|FlowControl|Gate true :!label _label
            (:Exit
              (if (Pawn|IsLocallyControlled)
                (|CameraFade _returnvalue)
                (CallFunction|ServerSpawnPawn _returnvalue)))))
        (:then_1
          (goto _label Open))))))

(event EventUnpossessed
  (params (OldController :type Controller%20Object%20Reference))
  (Actor|DestroyActor))

(fn ConstructionScript)