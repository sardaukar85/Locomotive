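; Helper actor that draws a curved laser pointer beam from spline meshes along a runtime-created spline.
; UpdateLaser uses sine-eased nested lerps to bend the beam from the forward vector toward the end location, then fits pooled meshes to the points.
; SetExpand plays or reverses a timeline that extends the beam when expansion is enabled.
; Setters snap or interpolate beam radius, plus color and opacity on one shared dynamic material.
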(event Custom|SetExpand
  (params (Set :type Boolean) (Time :type Float%20%28single-precision%29))
  (Components|Timeline|SetPlayRate (Variables|Default|GetExpandTimeline) (/ 1.0 Time))
  (if Set
    (bind _percent (Timeline|ExpandTimeline Play)
      (:Update
        (Variables|Pointer|SetExpandProgress _percent)))
    (else
      (Timeline|ExpandTimeline Reverse))))

(event EventBeginPlay
  (|CallParentFunction)
  ;[1 1 1] Prepare Pointer Spline
  (bind _returnvalue (AddComponent|AddSplineComponent false))
  (bind _output_get (Variables|Default|SetHelperSpline _returnvalue))
  (Spline|ClearSplinePoints _output_get true)
  (bind _returnvalue_2 (Rendering|Material|CreateDynamicMaterialInstance (Variables|Visuals|GetLaserMaterial) "None" "None" :!class /Script/Engine.KismetMaterialLibrary))
  (Variables|Pointer|SetSplineMaterial00 _returnvalue_2))

(event EventTick
  (params (DeltaSeconds :type Float%20%28single-precision%29))
  (|CallParentFunction DeltaSeconds))

(fn ConstructionScript)

(fn UpdateLaser
  (params (StartLocation :type Vector) (EndLocation :type Vector) (ForwardVector :type Vector))
  (bind _radiusindividualforeverysegment (Variables|Visuals|GetRadiusIndividualForEverySegment))
  (bind _helperspline (Variables|Default|GetHelperSpline))
  (bind _splinemeshes (Variables|Pointer|GetSplineMeshes))
  (bind _beamradiusstart (Variables|Visuals|GetBeamRadiusStart))
  (bind _beamradiusend (Variables|Visuals|GetBeamRadiusEnd))
  (bind _returnvalue (Utilities|Array|Length _splinemeshes))
  (bind _returnvalue_2 (Math|Conversions|ToFloat(Integer) _returnvalue))
  (LocalVariables|SetLocalStartLocation StartLocation)
  (Variables|Visuals|SetCurrentEndLocation (select (Variables|Settings|GetExapandable) (Math|Vector|Lerp(Vector) StartLocation EndLocation (Variables|Pointer|GetExpandProgress)) EndLocation))
  (LocalVariables|SetDistance (Math|Vector|Distance(Vector) (Variables|Visuals|GetCurrentEndLocation) (LocalVariables|GetLocalStartLocation)))
  (LocalVariables|SetLocalDesiredVector (+ (LocalVariables|GetLocalStartLocation) (* ForwardVector (LocalVariables|GetDistance))))
  (if (== (Spline|GetNumberOfSplinePoints (Variables|Default|GetHelperSpline)) 0)
    (for _index (range 0 (- (Variables|Settings|GetSplinePoints) 1))
      (Spline|AddSplinePoint (Variables|Default|GetHelperSpline) (Math|Vector|MakeVector (Math|Conversions|ToFloat(Integer) _index) 0.0 0.0) "Local" false)))
  (for _index_2 (range 0 (- (Variables|Settings|GetSplinePoints) 2))
    (LocalVariables|SetPointAlpha (|(sin((((x/y)*PI)*0.500000))) (Math|Conversions|ToFloat(Integer) _index_2) (Math|Conversions|ToFloat(Integer) (Variables|Settings|GetSplinePoints)) (Math|Trig|GetPI)))
    (Spline|SetLocationatSplinePoint (Variables|Default|GetHelperSpline) _index_2 (Math|Vector|Lerp(Vector) (Math|Vector|Lerp(Vector) (LocalVariables|GetLocalStartLocation) (LocalVariables|GetLocalDesiredVector) (LocalVariables|GetPointAlpha)) (Math|Vector|Lerp(Vector) (LocalVariables|GetLocalStartLocation) (Variables|Visuals|GetCurrentEndLocation) (LocalVariables|GetPointAlpha)) (LocalVariables|GetPointAlpha)) "Local" false))
  (Spline|SetLocationatSplinePoint (Variables|Default|GetHelperSpline) (- (Variables|Settings|GetSplinePoints) 1) (Variables|Visuals|GetCurrentEndLocation) "Local" true)
  (if (== (Utilities|Array|Length (Variables|Pointer|GetSplineMeshes)) 0)
    (for _index_3 (range 0 (- (Variables|Settings|GetSplinePoints) 1))
      (bind _returnvalue_3 (AddComponent|AddSplineMeshComponent true))
      (Utilities|Array|Add (Variables|Pointer|GetSplineMeshes) _returnvalue_3)
      (Rendering|Material|SetMaterial _returnvalue_3 0 (Variables|Pointer|GetSplineMaterial00))))
  (for _index_4 (range 0 (- (Variables|Settings|GetSplinePoints) 1))
    (SplineMesh|SetStartScale (Utilities|Array|Get(acopy) (Variables|Pointer|GetSplineMeshes) _index_4) (select _radiusindividualforeverysegment _beamradiusstart (CallFunction|LerpVector2D _beamradiusstart _beamradiusend (/ (Math|Conversions|ToFloat(Integer) _index_4) _returnvalue_2))) false :!class /Script/Engine.SplineMeshComponent)
    (SplineMesh|SetEndScale (Utilities|Array|Get(acopy) (Variables|Pointer|GetSplineMeshes) _index_4) (select _radiusindividualforeverysegment _beamradiusend (CallFunction|LerpVector2D _beamradiusstart _beamradiusend (/ (Math|Conversions|ToFloat(Integer) (+ _index_4 1)) _returnvalue_2))) false :!class /Script/Engine.SplineMeshComponent)
    (SplineMesh|SetStartandEnd (Utilities|Array|Get(acopy) (Variables|Pointer|GetSplineMeshes) _index_4) (.Location (Spline|GetLocationandTangentatSplinePoint _helperspline _index_4 "Local")) (.Tangent (Spline|GetLocationandTangentatSplinePoint _helperspline _index_4 "Local")) (.Location (Spline|GetLocationandTangentatSplinePoint _helperspline (+ _index_4 1) "Local")) (.Tangent (Spline|GetLocationandTangentatSplinePoint _helperspline (+ _index_4 1) "Local")) true :!class /Script/Engine.SplineMeshComponent)
    (Rendering|SetVisibility (Utilities|Array|Get(acopy) (Variables|Pointer|GetSplineMeshes) _index_4) true false)))

(fn SetLaserAttributes
  (params (InterpolationSpeed :type Float%20%28single-precision%29) (DeltaTime :type Float%20%28single-precision%29) (UseInterpolation :type Boolean) (WantedColor :type Linear%20Color%20Structure) (WantedOpacity :type Float%20%28single-precision%29) (RadiusStart :type Vector%202D%20Structure :default "(X=1.000000,Y=1.000000)") (RadiusEnd :type Vector%202D%20Structure :default "(X=1.000000,Y=1.000000)") (RadiusIndividualForEverySegment :type Boolean))
  (Visuals|SetLaserColor InterpolationSpeed DeltaTime UseInterpolation WantedColor)
  (Visuals|SetLaserOpacity InterpolationSpeed DeltaTime UseInterpolation WantedOpacity)
  (Visuals|SetLaserSize InterpolationSpeed DeltaTime UseInterpolation RadiusStart RadiusEnd RadiusIndividualForEverySegment))

(fn SetLaserColor
  (params (InterpolationSpeed :type Float%20%28single-precision%29) (DeltaTime :type Float%20%28single-precision%29) (UseInterpolation :type Boolean) (WantedColor :type Linear%20Color%20Structure))
  (Utilities|FlowControl|Sequence
    (:then_0
      (if UseInterpolation
        (Variables|Visuals|SetLaserColor (Class|KismetMathLibrary|CInterpto (Variables|Visuals|GetLaserColor) WantedColor DeltaTime InterpolationSpeed))
        (else
          (Variables|Visuals|SetLaserColor WantedColor))))
    (:then_1
      (Rendering|Material|SetVectorParameterValue (Variables|Pointer|GetSplineMaterial00) "Color" (Variables|Visuals|GetLaserColor) :!class /Script/Engine.MaterialInstanceDynamic))))

(fn SetLaserSize
  (params (InterpolationSpeed :type Float%20%28single-precision%29) (DeltaTime :type Float%20%28single-precision%29) (UseInterpolation :type Boolean) (RadiusStart :type Vector%202D%20Structure :default "(X=1.000000,Y=1.000000)") (RadiusEnd :type Vector%202D%20Structure :default "(X=1.000000,Y=1.000000)") (RadiusIndividualForEverySegment :type Boolean))
  (Variables|Visuals|SetRadiusIndividualForEverySegment RadiusIndividualForEverySegment)
  (if UseInterpolation
    (Variables|Visuals|SetBeamRadiusStart (Class|KismetMathLibrary|Vector2DInterpto (Variables|Visuals|GetBeamRadiusStart) RadiusStart DeltaTime InterpolationSpeed))
    (Variables|Visuals|SetBeamRadiusEnd (Class|KismetMathLibrary|Vector2DInterpto (Variables|Visuals|GetBeamRadiusEnd) RadiusEnd DeltaTime InterpolationSpeed))
    (else
      (Variables|Visuals|SetBeamRadiusStart RadiusStart)
      (Variables|Visuals|SetBeamRadiusEnd RadiusEnd))))

(fn SetLaserOpacity
  (params (InterpolationSpeed :type Float%20%28single-precision%29) (DeltaTime :type Float%20%28single-precision%29) (UseInterpolation :type Boolean) (WantedOpacity :type Float%20%28single-precision%29))
  (Utilities|FlowControl|Sequence
    (:then_0
      (if UseInterpolation
        (Variables|Visuals|SetLaserOpacity (Math|Interpolation|FInterpTo (Variables|Visuals|GetLaserOpacity) WantedOpacity DeltaTime InterpolationSpeed))
        (else
          (Variables|Visuals|SetLaserOpacity WantedOpacity))))
    (:then_1
      (Rendering|Material|SetScalarParameterValue (Variables|Pointer|GetSplineMaterial00) "Opacity" (Variables|Visuals|GetLaserOpacity) :!class /Script/Engine.MaterialInstanceDynamic))))